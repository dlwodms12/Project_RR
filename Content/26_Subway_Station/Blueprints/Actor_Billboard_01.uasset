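; Subway station billboard actor that animates a material panning parameter on a repeating cycle.
; The construction script uses a random MultiGate to choose between two billboard materials and creates a dynamic instance.
; After a random start delay, a timeline plays, pauses and restarts from the beginning each time it finishes.
; Tick writes the timeline value to the Panner_Time scalar parameter.
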(event EventBeginPlay
  (Utilities|FlowControl|Delay (Math|Random|RandomFloatinRange 0.0 2e+01))
  (bind _newtrack_0 (Timeline|Timeline_0 Play)
    (:Finished
      (Utilities|FlowControl|RetriggerableDelay 8.0)
      (Timeline|Timeline_0 PlayFromStart))))

(event Collision|EventActorBeginOverlap
  (params (OtherActor :type Actor%20Object%20Reference)))

(event EventTick
  (params (DeltaSeconds :type Float%20%28single-precision%29))
  (Rendering|Material|SetScalarParameterValue "Panner_Time" (stale EventBeginPlay _newtrack_0) :!class /Script/Engine.MaterialInstanceDynamic))

(fn ConstructionScript
  (Utilities|FlowControl|MultiGate true false -1
    (:Out%200
      (bind _returnvalue (Rendering|Material|CreateDynamicMaterialInstance 0 "/Game/Subway_Station/Materials/Mat_Billboard_01_Inst.Mat_Billboard_01_Inst" :!class /Script/Engine.PrimitiveComponent))
      (Variables|Default|SetMat _returnvalue))
    (:Out%201
      (bind _returnvalue_2 (Rendering|Material|CreateDynamicMaterialInstance 0 "/Game/Subway_Station/Materials/Mat_Billboard_04_Inst.Mat_Billboard_04_Inst" :!class /Script/Engine.PrimitiveComponent))
      (Variables|Default|SetMat _returnvalue_2))))