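; Subway station billboard actor that randomizes its material and panner timing.
; The construction script uses a random MultiGate to build a dynamic instance of one of two billboard materials on the Billboard02 component, stored as Mat.
; BeginPlay uses a second random MultiGate to set that instance's Panner_Time parameter to one of two values.
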(event EventBeginPlay
  (bind _mat (Variables|Default|GetMat))
  (Utilities|FlowControl|MultiGate true false -1
    (:Out%200
      (Rendering|Material|SetScalarParameterValue _mat "Panner_Time" 0.5 :!class /Script/Engine.MaterialInstanceDynamic))
    (:Out%201
      (Rendering|Material|SetScalarParameterValue _mat "Panner_Time" 1.0 :!class /Script/Engine.MaterialInstanceDynamic))))

(event Collision|EventActorBeginOverlap
  (params (OtherActor :type Actor%20Object%20Reference)))

(event EventTick
  (params (DeltaSeconds :type Float%20%28single-precision%29)))

(fn ConstructionScript
  (bind _billboard_02 (Variables|Default|GetBillboard_02))
  (Utilities|FlowControl|MultiGate true false -1
    (:Out%200
      (bind _returnvalue (Rendering|Material|CreateDynamicMaterialInstance _billboard_02 0 "/Game/Subway_Station/Materials/Mat_Billboard_02.Mat_Billboard_02" :!class /Script/Engine.PrimitiveComponent))
      (Variables|Default|SetMat _returnvalue))
    (:Out%201
      (bind _returnvalue_2 (Rendering|Material|CreateDynamicMaterialInstance _billboard_02 0 "/Game/Subway_Station/Materials/Mat_Billboard_05.Mat_Billboard_05" :!class /Script/Engine.PrimitiveComponent))
      (Variables|Default|SetMat _returnvalue_2))))