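; AI car that drives along the BP_SplinePath4 spline found in the level at BeginPlay.
; A timeline, with play rate scaled inversely to TimeToCompleteInSeconds, maps its alpha to spline distance and updates the car's location and rotation.
; Any hit on the Body sets Ragdoll on the BP_CustomMoveThirdPersonCharacter, regardless of what was struck.
; The crash sound plays through a DoOnce that resets after one second.
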(event OnComponentHit(Body)
  (params (HitComponent :type Primitive%20Component%20Object%20Reference) (OtherActor :type Actor%20Object%20Reference) (OtherComp :type Primitive%20Component%20Object%20Reference) (NormalImpulse :type Vector :default "0, 0, 0") (Hit :type Hit%20Result%20Structure%20%28by%20ref%29))
  (bind _returnvalue (Actor|GetActorOfClass "/Game/11_CustomMovement/Blueprints/BP_CustomMoveThirdPersonCharacter.BP_CustomMoveThirdPersonCharacter_C"))
  (Variables|/Game/11_CustomMovement/Blueprints/BP_CustomMoveThirdPersonCharacter.BP_CustomMoveThirdPersonCharacter_C|SetRagdoll _returnvalue true)
  (Utilities|FlowControl|DoOnce false :!label _label
    (:Completed
      (Audio|PlaySoundatLocation "/Game/Sound/SoundEffect/CarCrash.CarCrash" (Transformation|GetActorLocation) "0, 0, 0" 1.0 1.0 0.0 0 0 0 0)
      (Utilities|FlowControl|Delay 1.0)
      (goto _label Reset))))

(event Custom|Move%20Object
  (bind _spline_ref (Variables|Default|GetSpline%20REF))
  (bind _spline (Variables|/Game/AI_Car/BP_SplinePath4.BP_SplinePath4_C|GetSpline _spline_ref))
  (Components|Timeline|SetPlayRate (Variables|Default|GetMove%20Object%20T) (/ 0.2 (Variables|Default|GetTime%20To%20Complete%28In%20Seconds%29)))
  (bind _move_track (Timeline|Move%20Object%20T Play)
    (:Update
      (Transformation|SetActorTransform (Math|Transform|MakeTransform (Spline|GetLocationatDistanceAlongSpline _spline (Math|Float|Lerp 0.0 (Spline|GetSplineLength (Variables|/Game/AI_Car/BP_SplinePath4.BP_SplinePath4_C|GetSpline (Variables|Default|GetSpline%20REF))) _move_track) "World") (Spline|GetRotationatDistanceAlongSpline _spline (Math|Float|Lerp 0.0 (Spline|GetSplineLength (Variables|/Game/AI_Car/BP_SplinePath4.BP_SplinePath4_C|GetSpline (Variables|Default|GetSpline%20REF))) _move_track) "Local") "1.000000,1.000000,1.000000")))))

(event EventBeginPlay
  (bind _returnvalue (Actor|GetActorOfClass "/Game/AI_Car/BP_SplinePath4.BP_SplinePath4_C"))
  (Variables|Default|SetSpline%20REF _returnvalue)
  (CallFunction|MoveObject))

(fn ConstructionScript)