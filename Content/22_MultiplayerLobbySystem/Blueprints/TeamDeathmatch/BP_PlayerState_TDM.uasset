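; Player state for Team Deathmatch that carries the lobby's team choice, stored in the GameInstance, into the match.
; On BeginPlay, the listen-server host reads its red-team flag locally, while clients pass theirs to the server through ServerIsRedTeam.
; Both paths then have the TDM PlayerController spawn a red or blue character and register the player with the GameState's team lists.
; An owner check keeps dummy PlayerStates off the teams.
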(event Custom|ServerIsRedTeam
  (params (bInIsRedTeam :type Boolean))
  ;[0 0 0] Server | Setting the "bisRedTeam" bool from the GameInstance, passed by the lobby
  (Variables|Default|SetbIsRedTeam bInIsRedTeam)
  (CallFunction|HandleSpawningTeamBasedCharacter)
  (CallFunction|DetermineTeam))

(event Custom|IsRedTeam
  (bind _returnvalue (Components|GetOwner))
  (bind _returnvalue_2 (Game|GetGameInstance))
  ;[0 0 0] Server | Setting the "bisRedTeam" bool from the GameInstance, passed by the lobby
  (Utilities|IsValid _returnvalue
    (:Is%20Valid
      (bind _as플레이어_컨트롤러 (Utilities|Casting|CastToPlayerController _returnvalue))
      (if (Pawn|IsLocalPlayerController _as플레이어_컨트롤러)
        (Utilities|IsValid _returnvalue_2
          (:Is%20Valid
            (bind _asbp_game_instance (Utilities|Casting|CastToBP_GameInstance _returnvalue_2))
            (Variables|Default|SetbIsRedTeam (Variables|/Game/22_MultiplayerLobbySystem/Blueprints/BlueprintsUsedInAllMaps/BP_GameInstance.BP_GameInstance_C|GetbIsRedTeam _asbp_game_instance))
            (CallFunction|HandleSpawningTeamBasedCharacter)
            (CallFunction|DetermineTeam)))))))

(event Custom|HandleSpawningTeamBasedCharacter
  (bind _returnvalue (Components|GetOwner))
  ;[1 1 1] This handles spawning the team Characters. We need the RedTeam boolean so this might be the best place
  (Utilities|IsValid _returnvalue
    (:Is%20Valid
      (bind _asbp_player_controller_tdm (Utilities|Casting|CastToBP_PlayerController_TDM _returnvalue))
      (Default|ServerSpawnMe _asbp_player_controller_tdm (select (Variables|Default|GetbIsRedTeam) "/Game/22_MultiplayerLobbySystem/Blueprints/GamePlay/Characters/BP_Character_Red.BP_Character_Red_C" "/Game/22_MultiplayerLobbySystem/Blueprints/GamePlay/Characters/BP_Character_Blue.BP_Character_Blue_C")))))

(event Custom|DetermineTeam
  (bind _returnvalue (Game|GetGameState))
  (Utilities|IsValid (Components|GetOwner) ; Prevents Dummy PlayerState from being added
    (:Is%20Valid
      (Utilities|IsValid _returnvalue
        (:Is%20Valid
          (bind _asbp_game_state_tdm (Utilities|Casting|CastToBP_GameState_TDM _returnvalue))
          (Default|AddtoTeam _asbp_game_state_tdm self))))))

(event EventBeginPlay
  (bind _returnvalue (Game|GetGameInstance))
  ;[0 0 0] Clients and Server | tells the GameState to add us to the PlayerTeamLists and calls the bIsRedTeam Functions
  (|CallParentFunction)
  (Networking|SwitchHasAuthority
    (:Authority
      (CallFunction|IsRedTeam))
    (:Remote
      (Utilities|IsValid _returnvalue
        (:Is%20Valid
          (bind _asbp_game_instance (Utilities|Casting|CastToBP_GameInstance _returnvalue))
          (CallFunction|ServerIsRedTeam (Variables|/Game/22_MultiplayerLobbySystem/Blueprints/BlueprintsUsedInAllMaps/BP_GameInstance.BP_GameInstance_C|GetbIsRedTeam _asbp_game_instance)))))))

(fn ConstructionScript)