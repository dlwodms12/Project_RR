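; Lobby player controller that caches GameInstance and GameState references and marks the host's PlayerState as server for role-specific widgets.
; It bridges widget team-switch requests to the GameState, since clients cannot call its replicated functions directly.
; Kicks run on authority, removing the player from team lists and calling ClientDisconnect on their controller.
; ClientDisconnect optionally queues a reason in the GameInstance, disconnects and returns to the main menu.
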(event Custom|SetupReferences
  (bind _returnvalue (Game|GetGameState))
  (bind _returnvalue_2 (Game|GetGameInstance))
  ;[1 1 1] Save all kinds of important reference, so we don't have to cast all the time
  (Utilities|FlowControl|Sequence
    (:then_0
      (Utilities|IsValid _returnvalue_2
        (:Is%20Valid
          (bind _asbp_game_instance (Utilities|Casting|CastToBP_GameInstance _returnvalue_2))
          (Variables|Default|SetGameInstanceRef _asbp_game_instance))))
    (:then_1
      (Utilities|IsValid _returnvalue
        (:Is%20Valid
          (bind _asbp_game_state_lobby (Utilities|Casting|CastToBP_GameState_Lobby _returnvalue))
          (Variables|Default|SetGameStateRef _asbp_game_state_lobby))))))

(event Custom|KickPlayer
  (params (InPlayerState :type BP%20Player%20State%20Lobby%20Object%20Reference))
  (bind _gamestateref (Variables|Default|GetGameStateRef))
  ;[1 0 0] Server and Client | This will handle the KickButton Event from our Lobby. It will search the Player by the given ID and call the "ClientDisconnect" function on the matching client.
  ;;[0 1 0] Server | Kicks the given player by disconnecting him. Also removes him from all lists
  (Networking|SwitchHasAuthority
    (:Authority
      (Utilities|IsValid _gamestateref
        (:Is%20Valid
          (Default|RemovePlayerfromTeamList _gamestateref InPlayerState)
          (bind _asbp_player_controller_lobby (Utilities|Casting|CastToBP_PlayerController_Lobby (Components|GetOwner InPlayerState)))
          (CallFunction|ClientDisconnect _asbp_player_controller_lobby true "You were kicked!"))))))

(event Custom|ClientDisconnect
  (params (bInDisplayReason :type Boolean) (InReason :type Text))
  ;[1 0 0] Server and Client | This will handle the KickButton Event from our Lobby. It will search the Player by the given ID and call the "ClientDisconnect" function on the matching client.
  ;;[0 1 0] Client | Disconncets the Client with a specific reason. Also used for kicking a player. Sends him back to the MainMenu
  (Utilities|IsValid (Variables|Default|GetGameInstanceRef)
    (:Is%20Valid
      _)
    (:Is%20Not%20Valid
      (CallFunction|SetupReferences)))
  (if bInDisplayReason
    (Utilities|Array|Add (Variables|/Game/22_MultiplayerLobbySystem/Blueprints/BlueprintsUsedInAllMaps/BP_GameInstance.BP_GameInstance_C|GetPendingErrorMessage (Variables|Default|GetGameInstanceRef)) InReason))
  (Development|ExecuteConsoleCommand "Disconnect" self)
  (Default|TransitiontoMainMenu (Variables|Default|GetGameInstanceRef)))

(event Custom|ServerSwitchTeam
  ;[1 0 0] Clients and Server | These are Events that will call GameState function to change the Lists.
  ;;[0 1 1] Server | Tells the GameState to switch this Players Team. This is called from the Widget. We need this bridge because clients can't call replicated function on the GameState
  (Utilities|IsValid (Variables|Default|GetGameStateRef)
    (:Is%20Valid
      (bind _asbp_player_state_lobby (Utilities|Casting|CastToBP_PlayerState_Lobby (Variables|GetPlayerState)))
      (Default|SwitchTeam (Variables|Default|GetGameStateRef) _asbp_player_state_lobby))))

(event EventBeginPlay
  ;[1 0 0] Server | Since we want to display different widgets for server and clients, we need to save the "IsServer" somewhere. So we put this into our PlayerState
  (CallFunction|SetupReferences)
  (if (and (Networking|IsServer) (Pawn|IsLocalPlayerController))
    (bind _asbp_player_state_lobby (Utilities|Casting|CastToBP_PlayerState_Lobby (Variables|GetPlayerState)))
    (Variables|/Game/22_MultiplayerLobbySystem/Blueprints/Lobby/BP_PlayerState_Lobby.BP_PlayerState_Lobby_C|SetbIsServer _asbp_player_state_lobby true)))

(fn ConstructionScript)