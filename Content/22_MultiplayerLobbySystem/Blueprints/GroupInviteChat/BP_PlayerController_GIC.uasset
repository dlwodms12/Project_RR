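; Player controller for the multiplayer lobby project's chat and party system, handling all, group and whisper chat plus group invites.
; Server events build timestamped, colored messages, resolve players by Name or Name#ID, and deliver them through ClientReceiveMessage to the W_MainChat widget.
; Invites are validated on the server and shown via W_GroupInvite; accepting or leaving edits GroupMembers arrays and leader flags on each BP_PlayerState_GIC.
; It also answers help, player-list and ID requests with server messages.
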(event Custom|ServerRemovePlayerFromAllGroups
  ;[1 0 0] Server and Client | This handles our Group invites and keeps track of existing Groupmembers
  ;;[0 1 1] Server | This will handle removing the Player from his Group
  (GroupSystem|RemovePlayerStatefromGroup))

(event Custom|ServerSendGroupRequestByChat
  (params (InvitedPlayer :type Text))
  ;[1 0 0] Server and Client | This handles our Group invites and keeps track of existing Groupmembers
  ;;[1 0 1] Server | When sending the Request from Chat, we only pass the PlayerName
  (GroupSystem|SendGroupRequestFunction 0 InvitedPlayer))

(event Custom|ServerRequestAccepted
  (params (InvitingPlayerState :type BP%20Player%20State%20GIC%20Object%20Reference))
  ;[1 0 0] Server and Client | This handles our Group invites and keeps track of existing Groupmembers
  ;;[0 1 1] Server | This will handle adding the Player to the Group after accepting
  (GroupSystem|AddPlayerStatetoGroup InvitingPlayerState))

(event Custom|ClientReceiveMessage
  (params (InMessage :type F%20Chat%20Message%20Structure))
  (bind _chatwidget (Variables|WidgetReference|GetChatWidget))
  ;[1 0 0] Server and Clients | This is the Main logic of our Chat. The Server will construct the Message and send it to the given Group of Players (All/Group/Private). He will also try to find the Player we want to wisper to and return lists of players when using "/playerlist" commands etc. You will want to add more command features here!
  ;;[1 1 0] Client | This will tell the Chat widget to add a new MessageWidget with the given Message and color
  (Utilities|IsValid _chatwidget
    (:Is%20Valid
      (Default|AddMessagetoChat _chatwidget InMessage))))

(event Custom|ServerSendMessage
  (params (InReceivingPlayer :type Text) (InChatMode :type EChatMode%20Enum :default "NewEnumerator0") (InMessage :type Text))
  ;[1 0 0] Server and Clients | This is the Main logic of our Chat. The Server will construct the Message and send it to the given Group of Players (All/Group/Private). He will also try to find the Player we want to wisper to and return lists of players when using "/playerlist" commands etc. You will want to add more command features here!
  ;;[1 1 0] Server | We will construct a message with Time and Name of the Player and will chose the right method to send the Message based on the ChatMode
  (ChatSystem|HandleSendingChatMessage InReceivingPlayer InChatMode InMessage))

(event Custom|ServerChatGetPlayerList
  ;[1 0 0] Server and Clients | This is the Main logic of our Chat. The Server will construct the Message and send it to the given Group of Players (All/Group/Private). He will also try to find the Player we want to wisper to and return lists of players when using "/playerlist" commands etc. You will want to add more command features here!
  (ChatSystem|HandleChatGetPlayerList))

(event Custom|ServerSendGroupRequest
  (params (InvitedPlayerState :type Player%20State%20Object%20Reference))
  ;[1 0 0] Server and Client | This handles our Group invites and keeps track of existing Groupmembers
  ;;[0 1 1] Server | This will handle the GroupRequest
  (GroupSystem|SendGroupRequestFunction InvitedPlayerState))

(event Custom|ClientDisplayGroupInvite
  (params (InvitingPlayerState :type BP%20Player%20State%20GIC%20Object%20Reference))
  ;[1 0 0] Server and Client | This handles our Group invites and keeps track of existing Groupmembers
  ;;[0 1 1] Client | Invited Player | Creates the Invite Widget (if it is not already created) and passes the PlayerState of the Inviting Player, so we can display his name
  (Utilities|IsValid (Variables|WidgetReference|GetGroupInviteWidget)
    (:Is%20Valid
      (Variables|/Game/22_MultiplayerLobbySystem/Widgets/GroupInviteChat/W_GroupInvite.W_GroupInvite_C|SetInvitingPlayerState (Variables|WidgetReference|GetGroupInviteWidget) InvitingPlayerState))
    (:Is%20Not%20Valid
      (bind _returnvalue (UserInterface|CreateWidget "/Game/22_MultiplayerLobbySystem/Widgets/GroupInviteChat/W_GroupInvite.W_GroupInvite_C" (Game|GetPlayerController 0) InvitingPlayerState))
      (bind _output_get (Variables|WidgetReference|SetGroupInviteWidget _returnvalue))))
  (UserInterface|Viewport|AddtoViewport _output_get 0)
  (Input|SetInputModeGameandUI (Game|GetPlayerController 0) _output_get "DoNotLock" true false)
  (Variables|/Script/Engine.PlayerController|SetbShowMouseCursor (Game|GetPlayerController 0) true))

(event Custom|ServerHelpChat
  ;[1 0 0] Server and Clients | This is the Main logic of our Chat. The Server will construct the Message and send it to the given Group of Players (All/Group/Private). He will also try to find the Player we want to wisper to and return lists of players when using "/playerlist" commands etc. You will want to add more command features here!
  ;;[1 1 0] Server | This will ask the Server for a list of available commands. You need to add them here by hand at the moment
  (for _array_element (Variables|ChatSystem|GetChatCommands)
    (bind _outmessage (Utilities|CreateServerMessage _array_element)
      (:Outputs
        (ChatSystem|SendMessage self _outmessage)))))

(event Custom|ServerGetMyID
  ;[1 0 0] Server and Clients | This is the Main logic of our Chat. The Server will construct the Message and send it to the given Group of Players (All/Group/Private). He will also try to find the Player we want to wisper to and return lists of players when using "/playerlist" commands etc. You will want to add more command features here!
  ;;[1 1 0] Server | This will ask the Server for the PlayerID of the Client. You could get this directly in the Widget, but we want to not allow the Player Client to use the ServerMessage Macro
  (bind _outmessage (Utilities|CreateServerMessage (Utilities|Text|FormatText "Your PlayerID is: {PlayerID}" (Utilities|Text|ToText(Integer) (Variables|/Script/Engine.PlayerState|GetPlayerId (Variables|Default|GetPlayerState)))))
    (:Outputs
      (ChatSystem|SendMessage self _outmessage))))

(event EventBeginPlay
  (bind _playerstate (Variables|Default|GetPlayerState))
  ;[0 0 0] BeginPlay Messages for the Chat. Could use an Array here and just make an entry for each Message
  (|CallParentFunction)
  (Utilities|FlowControl|Sequence
    (:then_0
      (Utilities|IsValid _playerstate
        (:Is%20Valid
          (bind _asbp_player_state_gic (Utilities|Casting|CastToBP_PlayerState_GIC _playerstate))
          (Variables|Default|SetPlayerStateRef _asbp_player_state_gic))))
    (:then_1
      (Utilities|FlowControl|Sequence
        (:then_0
          (bind _outmessage (Utilities|CreateServerMessage "Welcome to eXi's Blueprint Networking Project.")
            (:Outputs
              (CallFunction|ClientReceiveMessage _outmessage))))
        (:then_1
          (bind _outmessage_2 (Utilities|CreateServerMessage "To use the Chat, press the 'Enter' - Key.")
            (:Outputs
              (CallFunction|ClientReceiveMessage _outmessage_2))))
        (:then_2
          (bind _outmessage_3 (Utilities|CreateServerMessage "To get a list of available Commands type /help")
            (:Outputs
              (CallFunction|ClientReceiveMessage _outmessage_3))))))))

(event Input|KeyboardEvents|Enter
  (params (Key :type Key%20Structure))
  (bind _chatwidget (Variables|WidgetReference|GetChatWidget))
  ;[1 0 0] Server and Clients | This is the Main logic of our Chat. The Server will construct the Message and send it to the given Group of Players (All/Group/Private). He will also try to find the Player we want to wisper to and return lists of players when using "/playerlist" commands etc. You will want to add more command features here!
  ;;[0 1 0] Press Enter to enable the chat if not already enabled
  (:Pressed
    (if (Variables|ChatSystem|GetbIsChatting)
      (Variables|ChatSystem|SetbIsChatting false)
      (else
        (Input|SetInputModeGameandUI self (Variables|/Game/22_MultiplayerLobbySystem/Widgets/GroupInviteChat/W_MainChat.W_MainChat_C|GetEnterChatMessage _chatwidget) "DoNotLock" true false)
        (Variables|ChatSystem|SetbIsChatting true)
        (Default|ShowChat _chatwidget)))))

(fn ConstructionScript
  (|CallParentFunction))

(fn SetupGameUI
  ;[1 1 1] In addition to MainHUD and InGameMenu, we want to add the Chat Widget
  (|CallParentFunction) ; Parent adds MainHUD and InGameMenu
  (if (Pawn|IsLocalPlayerController)
    (bind _returnvalue (UserInterface|CreateWidget "/Game/22_MultiplayerLobbySystem/Widgets/GroupInviteChat/W_MainChat.W_MainChat_C" self))
    (bind _output_get (Variables|WidgetReference|SetChatWidget _returnvalue))
    (UserInterface|Viewport|AddtoViewport _output_get 0)))

(fn ConstructMessage
  (params (InChatMode :type EChatMode%20Enum :default "NewEnumerator0") (InMessage :type Text))
  ;[1 1 1] We are building a message by first getting the SendingPlayersName and then chosing a color, based on the ChatMode. We also add the Time to the message which is UTC!
  (bind _outsendingplayername (Utilities|GetSendingPlayerName)
    (:Outputs
      (LocalVariables|SetSendingPlayerName _outsendingplayername)
      (bind _outcolor (ChatSystem|GetChatMessageColor InChatMode))
      (bind _output_get (LocalVariables|SetReturnMessage (Utilities|Text|FormatText "{Time}[{Name}]: {Message}" (Utilities|BuildTimeText) (LocalVariables|GetSendingPlayerName) InMessage)))
      (return (Utilities|Struct|MakeFChatMessage _output_get _outcolor)))))

(fn FindPlayerbyName
  (params (InPlayerName :type Text))
  (bind _returnvalue (Game|GetGameState))
  (bind _foundplayersarray (LocalVariables|GetFoundPlayersArray))
  (bind _output (Utilities|Array|Get(acopy) _foundplayersarray))
  (bind _returnvalue_2 (Components|GetOwner _output))
  ;[1 1 1] We check if the Player send a Playername together with an ID. If yes, we save them both and set the bool to true
  (bind (_outname _outid) (Utilities|HasIDinName InPlayerName)
    (:True
      (LocalVariables|SetbHasID true)
      (LocalVariables|SetPlayerName _outname)
      (LocalVariables|SetPlayerID _outid))
    (:False
      (LocalVariables|SetbHasID false)
      (LocalVariables|SetPlayerName InPlayerName)))
  ;[1 1 1] We reset the Variables for the new Search
  (Utilities|Array|Clear (LocalVariables|GetFoundPlayersArray))
  (LocalVariables|SetPlayersFound 0)
  ;[1 1 1] We use the PlayerArray of the GameState to search for the Player
  (Utilities|IsValid _returnvalue
    (:Is%20Valid
      (bind _asbp_game_state_base (Utilities|Casting|CastToBP_GameState_Base _returnvalue)
        (:then
          (for _array_element (Variables|/Script/Engine.GameState|GetPlayerArray _asbp_game_state_base)
            (Utilities|IsValid _array_element
              (:Is%20Valid
                ;[1 1 1] If we have a Playername AND an ID, we compare both and if they match, we add the Player to our Array. If we only have the Name, we only compare the Name. When we have an ID, we should only get one result though
                (bind _asbp_player_state_base (Utilities|Casting|CastToBP_PlayerState_Base _array_element))
                (if (or (Math|Boolean|ANDBoolean (LocalVariables|GetbHasID) (== (LocalVariables|GetPlayerID) (Variables|/Script/Engine.PlayerState|GetPlayerId _asbp_player_state_base)) (Utilities|Enum|Equal(Enum) (LocalVariables|GetPlayerName) (Utilities|Text|ToText(String) (Variables|/Script/Engine.PlayerState|GetPlayerName _asbp_player_state_base)))) (and (Utilities|Enum|Equal(Enum) (LocalVariables|GetPlayerName) (Utilities|Text|ToText(String) (Variables|/Script/Engine.PlayerState|GetPlayerName _asbp_player_state_base))) (not (LocalVariables|GetbHasID))))
                  (Math|Integer|IncrementInt (LocalVariables|GetPlayersFound)
                    (:%20%20
                      (Utilities|Array|Add (LocalVariables|GetFoundPlayersArray) _asbp_player_state_base)))))))
          ;[1 1 1] Check if we found a Player
          (if (> (LocalVariables|GetPlayersFound) 0)
            (if (> (LocalVariables|GetPlayersFound) 1)
              ;[1 1 1] We found more than 1 Player with the given name. I collapsed this to save some place
              (|MultiplePlayersFound
                (:Outpus
                  (return 0)))
              (else
                ;[1 1 1] If the PlayersFound Variable is 1, we found exactly one matching Player, so we get the Owner of the PlayerState (which is the PlayerController) and return it
                (Utilities|IsValid _output
                  (:Is%20Valid
                    (Utilities|IsValid _returnvalue_2
                      (:Is%20Valid
                        (bind _asbp_player_controller_gic (Utilities|Casting|CastToBP_PlayerController_GIC _returnvalue_2)
                          (:then
                            (return _asbp_player_controller_gic))
                          (:CastFailed
                            (return 0))))
                      (:Is%20Not%20Valid
                        _)))
                  (:Is%20Not%20Valid
                    _))
                (return 0)))
            (else
              ;[1 1 1] If the PlayersFound Variable is 0, we haven't found any Player with the given Name. So post a message to the Client which wanted to do something with the Player
              (bind _outmessage (Utilities|CreateServerMessage (Utilities|Text|FormatText "No Player found with name '{PlayerName}'!" (LocalVariables|GetPlayerName)))
                (:Outputs
                  (ChatSystem|SendMessage self _outmessage)
                  (return 0))))))
        (:CastFailed
          (return 0))))
    (:Is%20Not%20Valid
      (return 0))))

(fn RemovePlayerStatefromGroup
  (bind _playerstateref (Variables|Default|GetPlayerStateRef))
  (bind _playerstateref_2 (Variables|Default|GetPlayerStateRef))
  (bind _playerstateref_3 (Variables|Default|GetPlayerStateRef))
  (bind _playerstateref_4 (Variables|Default|GetPlayerStateRef))
  (bind _playerstateref_5 (Variables|Default|GetPlayerStateRef))
  ;[0 1 1] Server | If we are in a group, remove us from the Groups of all other group members and tell them to update their widget. Then, check if we are the Group Leader. If yes, make the first Player in our Group to the new GroupLeader and clear our GroupArray. If not, just clear the GroupArray. Also reset the bools that tell us if we are in a group and the groupleader. Then update our own GroupWidget. We also check if the one of the Members is the Server and tell him to update his Widget, because the OnRep function doesn't seem to get called correctly on the Server using a replicated Array
  (Utilities|IsValid _playerstateref
    (:Is%20Valid
      (if (Variables|/Game/22_MultiplayerLobbySystem/Blueprints/GroupInviteChat/BP_PlayerState_GIC.BP_PlayerState_GIC_C|GetbIsInGroup _playerstateref)
        (for _array_element (Variables|/Game/22_MultiplayerLobbySystem/Blueprints/GroupInviteChat/BP_PlayerState_GIC.BP_PlayerState_GIC_C|GetGroupMembers _playerstateref)
          ;;[0 1 0] Get the current PlayerState and save it in the Temp Variable. This just helps us keeping this function clean
          (bind _output_get (LocalVariables|SetCurrentPlayerState _array_element))
          (Utilities|IsValid _output_get
            (:Is%20Valid
              ;;[0 1 0] Remove this Players PlayerState from the current Players Group (not his own!)
              (if (!= (Variables|Default|GetPlayerStateRef) (LocalVariables|GetCurrentPlayerState))
                (Utilities|Array|RemoveItem (Variables|/Game/22_MultiplayerLobbySystem/Blueprints/GroupInviteChat/BP_PlayerState_GIC.BP_PlayerState_GIC_C|GetGroupMembers (LocalVariables|GetCurrentPlayerState)) (Variables|Default|GetPlayerStateRef))
                ;;[0 1 0] If we have one or less members in this Players Group (means he is alone in his group), we completely revoke the Group
                (if (< (Utilities|Array|Length (Variables|/Game/22_MultiplayerLobbySystem/Blueprints/GroupInviteChat/BP_PlayerState_GIC.BP_PlayerState_GIC_C|GetGroupMembers (LocalVariables|GetCurrentPlayerState))) 2)
                  (Utilities|Array|Clear (Variables|/Game/22_MultiplayerLobbySystem/Blueprints/GroupInviteChat/BP_PlayerState_GIC.BP_PlayerState_GIC_C|GetGroupMembers (LocalVariables|GetCurrentPlayerState)))
                  (Variables|/Game/22_MultiplayerLobbySystem/Blueprints/GroupInviteChat/BP_PlayerState_GIC.BP_PlayerState_GIC_C|SetbIsInGroup (LocalVariables|GetCurrentPlayerState) false)
                  (Variables|/Game/22_MultiplayerLobbySystem/Blueprints/GroupInviteChat/BP_PlayerState_GIC.BP_PlayerState_GIC_C|SetbIsGroupLeader (LocalVariables|GetCurrentPlayerState) false))
                (Variables|/Game/22_MultiplayerLobbySystem/Blueprints/GroupInviteChat/BP_PlayerState_GIC.BP_PlayerState_GIC_C|SetGroupMembers (LocalVariables|GetCurrentPlayerState) (Variables|/Game/22_MultiplayerLobbySystem/Blueprints/GroupInviteChat/BP_PlayerState_GIC.BP_PlayerState_GIC_C|GetGroupMembers (LocalVariables|GetCurrentPlayerState)))))))
        ;;[0 1 0] If this Player was the Group leader and the group was larger than 2 people (so we have a group remaining and not a single player), give these rights to the first Player in the remaining Group
        (Utilities|IsValid _playerstateref_2
          (:Is%20Valid
            (if (and (Variables|/Game/22_MultiplayerLobbySystem/Blueprints/GroupInviteChat/BP_PlayerState_GIC.BP_PlayerState_GIC_C|GetbIsGroupLeader _playerstateref_2) (> (Utilities|Array|Length (Variables|/Game/22_MultiplayerLobbySystem/Blueprints/GroupInviteChat/BP_PlayerState_GIC.BP_PlayerState_GIC_C|GetGroupMembers _playerstateref_2)) 2))
              (Utilities|IsValid (Utilities|Array|Get(acopy) (Variables|/Game/22_MultiplayerLobbySystem/Blueprints/GroupInviteChat/BP_PlayerState_GIC.BP_PlayerState_GIC_C|GetGroupMembers _playerstateref_2) 1)
                (:Is%20Valid
                  (Variables|/Game/22_MultiplayerLobbySystem/Blueprints/GroupInviteChat/BP_PlayerState_GIC.BP_PlayerState_GIC_C|SetbIsGroupLeader (Utilities|Array|Get(acopy) (Variables|/Game/22_MultiplayerLobbySystem/Blueprints/GroupInviteChat/BP_PlayerState_GIC.BP_PlayerState_GIC_C|GetGroupMembers _playerstateref_2) 1) true))))
            ;;[0 1 0.006] Clears this Players Group and sets the bools to false
            (Utilities|IsValid _playerstateref_3
              (:Is%20Valid
                (Utilities|Array|Clear (Variables|/Game/22_MultiplayerLobbySystem/Blueprints/GroupInviteChat/BP_PlayerState_GIC.BP_PlayerState_GIC_C|GetGroupMembers _playerstateref_3))
                (Variables|/Game/22_MultiplayerLobbySystem/Blueprints/GroupInviteChat/BP_PlayerState_GIC.BP_PlayerState_GIC_C|SetbIsInGroup _playerstateref_5 false)
                (Variables|/Game/22_MultiplayerLobbySystem/Blueprints/GroupInviteChat/BP_PlayerState_GIC.BP_PlayerState_GIC_C|SetbIsGroupLeader _playerstateref_5 false)
                (Variables|/Game/22_MultiplayerLobbySystem/Blueprints/GroupInviteChat/BP_PlayerState_GIC.BP_PlayerState_GIC_C|SetGroupMembers _playerstateref_4 (Variables|/Game/22_MultiplayerLobbySystem/Blueprints/GroupInviteChat/BP_PlayerState_GIC.BP_PlayerState_GIC_C|GetGroupMembers _playerstateref_4))))))
        (else
          ;;[1 1 0] Interacting with the chat system
          (bind _outmessage (Utilities|CreateServerMessage "You are not in a Group")
            (:Outputs
              (ChatSystem|SendMessage self _outmessage))))))))

(fn SendGroupRequestFunction
  (params (InPlayerState :type Player%20State%20Object%20Reference) (InPlayerName :type Text))
  (bind _playerstateref (Variables|Default|GetPlayerStateRef))
  ;[1 1 1] If we get a PlayerState passed, save it and get the PlayerController from it (The Owner)
  (Utilities|IsValid InPlayerState
    (:Is%20Valid
      (bind _output_get (LocalVariables|SetInvitedPlayerState InPlayerState))
      (Utilities|IsValid (Components|GetOwner _output_get)
        (:Is%20Valid
          (bind _asbp_player_controller_gic (Utilities|Casting|CastToBP_PlayerController_GIC (Components|GetOwner _output_get)))
          (LocalVariables|SetInvitedPlayerController _asbp_player_controller_gic))))
    (:Is%20Not%20Valid
      ;[1 1 1] If we only get a Name, we need to search the Player with the Name. Once we did that, save the PlayerController and the PlayerState again
      (bind _outplayercontroller (ChatSystem|FindPlayerbyName InPlayerName))
      (bind _output_get_2 (LocalVariables|SetInvitedPlayerController _outplayercontroller))
      (Utilities|IsValid _output_get_2
        (:Is%20Valid
          (Utilities|IsValid (Variables|/Script/Engine.Controller|GetPlayerState _output_get_2)
            (:Is%20Valid
              (bind _asbp_player_state_gic (Utilities|Casting|CastToBP_PlayerState_GIC (Variables|/Script/Engine.Controller|GetPlayerState _output_get_2)))
              (LocalVariables|SetInvitedPlayerState _asbp_player_state_gic)))))))
  ;[1 1 1] Check if the INVITING Player is already in a Group, because then he needs to be the leader
  (Utilities|IsValid _playerstateref
    (:Is%20Valid
      (bind _output_get_3 (LocalVariables|SetInvitingPlayerState _playerstateref))
      (if (Variables|/Game/22_MultiplayerLobbySystem/Blueprints/GroupInviteChat/BP_PlayerState_GIC.BP_PlayerState_GIC_C|GetbIsInGroup _output_get_3)
        ;[1 1 1] Are we the leader of the group?
        (if (Variables|/Game/22_MultiplayerLobbySystem/Blueprints/GroupInviteChat/BP_PlayerState_GIC.BP_PlayerState_GIC_C|GetbIsGroupLeader (LocalVariables|GetInvitingPlayerState))
          ;[1 1 1] Trying to invite ourself?
          (Utilities|ComparePlayerIDs (LocalVariables|GetInvitingPlayerState) (LocalVariables|GetInvitedPlayerState) :!label _label
            (:Same
              ;[1 1 0] Interact with the Chat System
              (bind _outmessage (Utilities|CreateServerMessage "You can't invite yourself!")
                (:Outputs
                  (ChatSystem|SendMessage self _outmessage))))
            (:NotTheSame
              ;[1 1 1] Player we want to invite already in OUR group?
              (Utilities|IsAlreadyinGroup (LocalVariables|GetInvitedPlayerState)
                (:True
                  (bind _outmessage_2 (Utilities|CreateServerMessage "Player is already in your group!")
                    (:Outputs
                      (ChatSystem|SendMessage self _outmessage_2))))
                (:False
                  ;[1 1 1] Make sure the Player is not in another group
                  (bind _asbp_player_state_gic_2 (Utilities|Casting|CastToBP_PlayerState_GIC (LocalVariables|GetInvitedPlayerState)))
                  (if (Variables|/Game/22_MultiplayerLobbySystem/Blueprints/GroupInviteChat/BP_PlayerState_GIC.BP_PlayerState_GIC_C|GetbIsInGroup _asbp_player_state_gic_2)
                    (bind _outmessage_3 (Utilities|CreateServerMessage "Player is already in a group!")
                      (:Outputs
                        (ChatSystem|SendMessage self _outmessage_3)))
                    (else
                      ;[1 1 1] All checks succeeded, invite the Player
                      (CallFunction|ClientDisplayGroupInvite (LocalVariables|GetInvitedPlayerController) (LocalVariables|GetInvitingPlayerState))))))))
          (else
            (bind _outmessage_4 (Utilities|CreateServerMessage "You are not the leader!")
              (:Outputs
                (ChatSystem|SendMessage self _outmessage_4)))))
        (else
          (goto _label))))))

(fn AddPlayerStatetoGroup
  (params (InPlayerState :type BP%20Player%20State%20GIC%20Object%20Reference))
  (bind _playerstateref (Variables|Default|GetPlayerStateRef))
  ;[0 1 1] Server | Invited Player | When the Player accepts the invite, we check if the inviting person is already in a group, if not, make him the group leader and set him to be in a group. We also add him to his own Group Array, because we will use ONE overall group for all group members of that specific group, and this will be the one of the GroupLeader. Then we iterate through his array, and set everyone elses array to his one
  (bind _output_get (LocalVariables|SetInvitingPlayerState InPlayerState))
  (Utilities|IsValid _output_get
    (:Is%20Valid
      ;;[0 1 0] Check if the inviting person is already in a group. If not, add him to the overall group
      (if (Variables|/Game/22_MultiplayerLobbySystem/Blueprints/GroupInviteChat/BP_PlayerState_GIC.BP_PlayerState_GIC_C|GetbIsInGroup (LocalVariables|GetInvitingPlayerState))
        _
        (else
          (Utilities|Array|Add (Variables|/Game/22_MultiplayerLobbySystem/Blueprints/GroupInviteChat/BP_PlayerState_GIC.BP_PlayerState_GIC_C|GetGroupMembers (LocalVariables|GetInvitingPlayerState)) (LocalVariables|GetInvitingPlayerState))
          ;;[0 1 0] Set GroupLeader bools
          (Variables|/Game/22_MultiplayerLobbySystem/Blueprints/GroupInviteChat/BP_PlayerState_GIC.BP_PlayerState_GIC_C|SetbIsInGroup (LocalVariables|GetInvitingPlayerState) true)
          (Variables|/Game/22_MultiplayerLobbySystem/Blueprints/GroupInviteChat/BP_PlayerState_GIC.BP_PlayerState_GIC_C|SetbIsGroupLeader (LocalVariables|GetInvitingPlayerState) true)))
      ;;[0 1 0] Add new Player to GroupLeader Array
      (Utilities|Array|Add (Variables|/Game/22_MultiplayerLobbySystem/Blueprints/GroupInviteChat/BP_PlayerState_GIC.BP_PlayerState_GIC_C|GetGroupMembers (LocalVariables|GetInvitingPlayerState)) (Variables|Default|GetPlayerStateRef))
      ;;[0 1 0] Set the Group of all other Players to the new updated array of the GroupLeader
      (for _array_element (Variables|/Game/22_MultiplayerLobbySystem/Blueprints/GroupInviteChat/BP_PlayerState_GIC.BP_PlayerState_GIC_C|GetGroupMembers (LocalVariables|GetInvitingPlayerState))
        (Utilities|IsValid _array_element
          (:Is%20Valid
            (Variables|/Game/22_MultiplayerLobbySystem/Blueprints/GroupInviteChat/BP_PlayerState_GIC.BP_PlayerState_GIC_C|SetGroupMembers _array_element (Variables|/Game/22_MultiplayerLobbySystem/Blueprints/GroupInviteChat/BP_PlayerState_GIC.BP_PlayerState_GIC_C|GetGroupMembers (LocalVariables|GetInvitingPlayerState))))))
      ;;[0 1 0] Sets the important Group Bools for the InvitedPlayer
      (Utilities|IsValid _playerstateref
        (:Is%20Valid
          (Variables|/Game/22_MultiplayerLobbySystem/Blueprints/GroupInviteChat/BP_PlayerState_GIC.BP_PlayerState_GIC_C|SetbIsInGroup _playerstateref true)
          (Variables|/Game/22_MultiplayerLobbySystem/Blueprints/GroupInviteChat/BP_PlayerState_GIC.BP_PlayerState_GIC_C|SetbIsGroupLeader _playerstateref false))))))

(fn GetChatMessageColor
  (params (InChatMode :type EChatMode%20Enum :default "NewEnumerator0"))
  (switch Utilities|FlowControl|Switch|SwitchonEChatMode InChatMode
    (:NewEnumerator0
      (return "(R=0.760524,G=0.768151,B=0.775822,A=1.000000)"))
    (:NewEnumerator1
      (return "(R=0.000000,G=0.730000,B=0.083584,A=1.000000)"))
    (:NewEnumerator2
      (return "(R=1.000000,G=0.000000,B=0.565984,A=1.000000)"))))

(fn HandleSendingChatMessage
  (params (InReceivingPlayer :type Text) (InChatMode :type EChatMode%20Enum :default "NewEnumerator0") (InMessage :type Text))
  (LocalVariables|SetReceivingPlayer InReceivingPlayer)
  (LocalVariables|SetChatMode InChatMode)
  (bind _outmessage (ChatSystem|ConstructMessage InChatMode InMessage))
  (LocalVariables|SetMessage _outmessage)
  (switch Utilities|FlowControl|Switch|SwitchonEChatMode (LocalVariables|GetChatMode)
    (:NewEnumerator0
      (ChatSystem|SendMessagetoAllChat (LocalVariables|GetMessage)))
    (:NewEnumerator1
      (ChatSystem|SendMessagetoGroup (LocalVariables|GetMessage)))
    (:NewEnumerator2
      (ChatSystem|SendMessagetoPlayer (LocalVariables|GetMessage) (LocalVariables|GetReceivingPlayer)))))

(fn SendMessagetoAllChat
  (params (InMessage :type F%20Chat%20Message%20Structure))
  ;[1 1 0] Server | Sending to AllChat means that we will send a message to every PlayerController. So we get all Actors of Class PlayerController and call the SendMessage Function on them
  (bind _outactors (Actor|GetAllActorsOfClass "BP_PlayerController_GIC_C"))
  (for _array_element _outactors
    (Utilities|IsValid _array_element
      (:Is%20Valid
        (ChatSystem|SendMessage _array_element InMessage)))))

(fn SendMessagetoGroup
  (params (InMessage :type F%20Chat%20Message%20Structure))
  (bind _playerstate (Variables|Default|GetPlayerState))
  ;[1 1 0] Server | Sending to the Group means that we only look at the Array which contains our Group Members. Check if we are part of a group, if yes then we iterate through the GroupMembers and call the SendMessage function on them
  (LocalVariables|SetMessage InMessage)
  (Utilities|IsValid _playerstate
    (:Is%20Valid
      (bind _asbp_player_state_gic (Utilities|Casting|CastToBP_PlayerState_GIC _playerstate))
      (if (Variables|/Game/22_MultiplayerLobbySystem/Blueprints/GroupInviteChat/BP_PlayerState_GIC.BP_PlayerState_GIC_C|GetbIsInGroup _asbp_player_state_gic)
        (for _array_element (Variables|/Game/22_MultiplayerLobbySystem/Blueprints/GroupInviteChat/BP_PlayerState_GIC.BP_PlayerState_GIC_C|GetGroupMembers _asbp_player_state_gic)
          (Utilities|IsValid _array_element
            (:Is%20Valid
              (bind _asbp_player_state_gic_2 (Utilities|Casting|CastToBP_PlayerState_GIC _array_element))
              (Utilities|IsValid (Components|GetOwner _asbp_player_state_gic_2)
                (:Is%20Valid
                  (bind _asbp_player_controller_gic (Utilities|Casting|CastToBP_PlayerController_GIC (Components|GetOwner _asbp_player_state_gic_2)))
                  (ChatSystem|SendMessage _asbp_player_controller_gic (LocalVariables|GetMessage)))))))
        (else
          (bind _outmessage (Utilities|CreateServerMessage "You are not in a Group!")
            (:Outputs
              (ChatSystem|SendMessage self _outmessage))))))))

(fn SendMessagetoPlayer
  (params (InMessage :type F%20Chat%20Message%20Structure) (InPlayerName :type Text))
  ;[1 1 0] Sending to a Player means we check if we can find the Player and then send him the message and also ourself
  (LocalVariables|SetMessage InMessage)
  (bind _outplayercontroller (ChatSystem|FindPlayerbyName InPlayerName))
  (Utilities|IsValid _outplayercontroller
    (:Is%20Valid
      (ChatSystem|SendMessage _outplayercontroller (LocalVariables|GetMessage))
      (ChatSystem|SendMessage self (LocalVariables|GetMessage)))))

(fn SendMessage
  (params (InPlayerController :type BP%20Player%20Controller%20GIC%20Object%20Reference) (InMessage :type F%20Chat%20Message%20Structure))
  (CallFunction|ClientReceiveMessage InPlayerController InMessage))

(fn HandleChatGetPlayerList
  (bind _returnvalue (Game|GetGameState))
  ;[1 1 0] Server | This will ask the Server for a List of all Players. We will get the PlayerArray of the Gamestate and post a list of Playername and ID of all Players
  (Utilities|IsValid _returnvalue
    (:Is%20Valid
      (bind _outmessage (Utilities|CreateServerMessage (Utilities|Text|FormatText "There are {Number} Players:" (Utilities|Text|ToText(Integer) (Utilities|Array|Length (Variables|/Script/Engine.GameState|GetPlayerArray _returnvalue)))))
        (:Outputs
          (ChatSystem|SendMessage self _outmessage)
          (for _array_element (Variables|/Script/Engine.GameState|GetPlayerArray (Game|GetGameState))
            (Utilities|IsValid _array_element
              (:Is%20Valid
                (bind _asbp_player_state_base (Utilities|Casting|CastToBP_PlayerState_Base _array_element))
                (bind _outmessage_2 (Utilities|CreateServerMessage (Utilities|Text|FormatText "{PlayerName}#{ID}" (Utilities|Text|ToText(String) (Variables|/Script/Engine.PlayerState|GetPlayerName _asbp_player_state_base)) (Utilities|Text|ToText(Integer) (Variables|/Script/Engine.PlayerState|GetPlayerId _asbp_player_state_base))))
                  (:Outputs
                    (ChatSystem|SendMessage self _outmessage_2)))))))))))