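; Base platform actor that carries a collectable in a multiplayer level.
; On BeginPlay, the server spawns a BP_Collectable at the CollectablePosition component, passes itself as PlatformRef and stores the new actor in CollectableRef.
; RespawnCollectable, meant for game resets, repeats that authority-only spawn when the stored collectable is no longer valid.
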(event EventBeginPlay
  ;[1 1 1] Server | Spawns a new Collectable at the CollectablePosition
  (Networking|SwitchHasAuthority
    (:Authority
      (bind _returnvalue (Game|SpawnActorfromClass "/Game/22_MultiplayerLobbySystem/Blueprints/GamePlay/BP_Collectable.BP_Collectable_C" (Transformation|GetWorldTransform (Variables|Default|GetCollectablePosition)) "AlwaysSpawn" "OverrideRootScale" 0 self 0))
      (Variables|Default|SetCollectableRef _returnvalue))))

(fn ConstructionScript)

(fn RespawnCollectable
  ;[1 1 1] If the Collectable, which the Platform carries, is gone, respawn one when the Game gets resetted
  (Networking|SwitchHasAuthority
    (:Authority
      (Utilities|IsValid (Variables|Default|GetCollectableRef)
        (:Is%20Not%20Valid
          (bind _returnvalue (Game|SpawnActorfromClass "/Game/22_MultiplayerLobbySystem/Blueprints/GamePlay/BP_Collectable.BP_Collectable_C" (Transformation|GetWorldTransform (Variables|Default|GetCollectablePosition)) "AlwaysSpawn" "OverrideRootScale" 0 self 0))
          (Variables|Default|SetCollectableRef _returnvalue))))))