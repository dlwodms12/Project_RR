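; BP_Collectable is a floating pickup that awards score to the player who touches it in a multiplayer game.
; A Timeline started on BeginPlay offsets its Z from the start position to animate the hover.
; Mesh overlap is handled once, on authority only, calling AddScore on the overlapping character's PlayerState.
; With a valid PlatformRef, it then clears that platform's CollectableRef and destroys itself.
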(event OnComponentBeginOverlap(StaticMesh)
  (params (OverlappedComponent :type Primitive%20Component%20Object%20Reference) (OtherActor :type Actor%20Object%20Reference) (OtherComp :type Primitive%20Component%20Object%20Reference) (OtherBodyIndex :type Integer) (bFromSweep :type Boolean) (SweepResult :type Hit%20Result%20Structure%20%28by%20ref%29))
  (bind _platformref (Variables|Default|GetPlatformRef))
  ;[1 1 1] Server | When something overlaps the  Collectable Model, we check if we are the server and if the Overlapping Actor is valid. We also make sure that we only call this once. After that we cast to the PlayerCharacter BaseClass to make sure that a Player overlapped and to get the Controller of that Player. Then we call AddScore from the PC and destroy the collectable
  (Networking|SwitchHasAuthority
    (:Authority
      (Utilities|FlowControl|DoOnce false
        (:Completed
          (Utilities|IsValid OtherActor
            (:Is%20Valid
              (bind _asbp_character_base (Utilities|Casting|CastToBP_Character_Base OtherActor))
              (Utilities|IsValid (Variables|/Script/Engine.Pawn|GetPlayerState _asbp_character_base)
                (:Is%20Valid
                  (bind _asbp_player_state_base (Utilities|Casting|CastToBP_PlayerState_Base (Variables|/Script/Engine.Pawn|GetPlayerState _asbp_character_base)))
                  (Default|AddScore _asbp_player_state_base)
                  (Utilities|IsValid _platformref
                    (:Is%20Valid
                      (Variables|/Game/22_MultiplayerLobbySystem/Blueprints/GamePlay/BP_Platform_Base.BP_Platform_Base_C|SetCollectableRef _platformref 0)
                      (Actor|DestroyActor))))))))))))

(event EventBeginPlay
  ;[1 1 1] This will "Animate" the Model of the Collectable. It will use a Timeline to change the Z Value, so it seems like it is flowting
  (Variables|Default|SetStartPosition (Transformation|GetActorLocation))
  (bind _positionz (Timeline|LocationTimeLine Play)
    (:Update
      (Transformation|SetActorLocation (Math|Vector|MakeVector (.x (Variables|Default|GetStartPosition)) (.y (Variables|Default|GetStartPosition)) (+ (.z (Variables|Default|GetStartPosition)) _positionz)) false false))))

(fn ConstructionScript)