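; Base GameMode for the multiplayer lobby system that enforces a player limit when players join.
; BeginPlay reads MaxNumPlayers from the options string.
; PostLogin increments the player count and disconnects players over the limit through their BP_PlayerController_Base with a "Server is full!" reason.
; Otherwise it multicasts a scoreboard refresh through BP_GameState_Base and calls the custom ClientPostLogin on the new player's controller.
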(event EventPostLogin
  (params (NewPlayer :type Player%20Controller%20Object%20Reference))
  (bind _returnvalue (Game|GetGameState))
  ;[1 1 1] If Server is full, remove the Player directly and tell him
  (bind _result (Math|Integer|IncrementInt (Variables|Default|GetCurrentNumberOfPlayers))
    (:%20%20
      (if (and (> _result (Variables|Default|GetMaxNumPlayers)) (> (Variables|Default|GetCurrentNumberOfPlayers) 1))
        (bind _asbp_player_controller_base (Utilities|Casting|CastToBP_PlayerController_Base NewPlayer))
        (Default|ClientDisconnect _asbp_player_controller_base true "Server is full!")
        (else
          ;[1 1 1] When a new Player joins tell everybody to update their Scoreboard for the fact if someone has it open just now. Also call the selfmade "ClientPostLogin" version on the PlayerController of the new Player
          (Utilities|FlowControl|Sequence
            (:then_0
              (Utilities|IsValid _returnvalue
                (:Is%20Valid
                  (bind _asbp_game_state_base (Utilities|Casting|CastToBP_GameState_Base _returnvalue))
                  (Default|MulticastUpdateScoreboard _asbp_game_state_base))))
            (:then_1
              (bind _asbp_player_controller_base_2 (Utilities|Casting|CastToBP_PlayerController_Base NewPlayer))
              (Default|ClientPostLogin _asbp_player_controller_base_2))))))))

(event EventBeginPlay
  (Variables|Default|SetMaxNumPlayers (Math|Conversions|ToInteger(Byte) (Class|GameplayStatics|ParseOption (Variables|Default|GetOptionsString) "MaxNumPlayers"))))

(fn ConstructionScript)