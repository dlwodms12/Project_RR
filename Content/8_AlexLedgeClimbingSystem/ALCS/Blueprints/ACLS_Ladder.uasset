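; Climbable ladder actor for the ledge climbing system, built procedurally in the construction script from a vertical end point.
; It stacks mesh segments, scales the climb volumes to that height and line-traces at the top to place the exit triggers and top mesh.
; A failed trace shows a bad-ladder warning, which disables the ladder at BeginPlay.
; Overlap volumes set ladder state on the character and trigger climbing off or down at the top.
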(event OnComponentEndOverlap(TopClimbDownTrigger)
  (params (OverlappedComponent :type Primitive%20Component%20Object%20Reference) (OtherActor :type Actor%20Object%20Reference) (OtherComp :type Primitive%20Component%20Object%20Reference) (OtherBodyIndex :type Integer))
  ;[1 1 1] Gave up on climbing down the ladder
  (Variables|Default|SetbTopClimbDownTrigger false)
  (bind _asaledgeclimbsystemcharacter_c (Utilities|Casting|CastTo OtherActor))
  (Variables|Default|SetbLadderTopVolume _asaledgeclimbsystemcharacter_c false)
  (Rendering|SetVisibility (Variables|Default|GetTextClimbDown) false false))

(event OnComponentBeginOverlap(LadderVolumeMesh)
  (params (OverlappedComponent :type Primitive%20Component%20Object%20Reference) (OtherActor :type Actor%20Object%20Reference) (OtherComp :type Primitive%20Component%20Object%20Reference) (OtherBodyIndex :type Integer) (bFromSweep :type Boolean) (SweepResult :type Hit%20Result%20Structure%20%28by%20ref%29))
  ;[1 1 1] Ladder In and Out
  (if (not (Variables|Default|GetbDisabled))
    (if (not (Variables|Default|GetbTopClimbDownTrigger))
      (if (not (Variables|Default|GetbTopGetOutTrigger))
        (bind _asaledgeclimbsystemcharacter_c (Utilities|Casting|CastTo OtherActor))
        ;;[1 1 1] If the ladder is at the right height
        (if (<= (.Z (Math|Vector|BreakVector (Transformation|GetActorLocation))) (+ (.Z (Math|Vector|BreakVector (Transformation|GetActorLocation _asaledgeclimbsystemcharacter_c))) 6e+01))
          (if (not (Variables|Default|GetbMovingBackward _asaledgeclimbsystemcharacter_c))
            (Variables|Default|SetbInLadderVolume _asaledgeclimbsystemcharacter_c true)
            (Variables|Default|SetbInLadderVolume true)
            (Variables|Default|SetLadderToClimb _asaledgeclimbsystemcharacter_c self)
            (Variables|Default|SetbLadderPositioned _asaledgeclimbsystemcharacter_c false)))))))

(event OnComponentBeginOverlap(TopGetOutTrigger)
  (params (OverlappedComponent :type Primitive%20Component%20Object%20Reference) (OtherActor :type Actor%20Object%20Reference) (OtherComp :type Primitive%20Component%20Object%20Reference) (OtherBodyIndex :type Integer) (bFromSweep :type Boolean) (SweepResult :type Hit%20Result%20Structure%20%28by%20ref%29))
  ;[1 1 1] Start to get out at the top of the ladder
  (if (not (Variables|Default|GetbDisabled))
    (Variables|Default|SetbTopGetOutTrigger true)
    (if (not (Variables|Default|GetbTopClimbDownTrigger))
      (bind _asaledgeclimbsystemcharacter_c (Utilities|Casting|CastTo OtherActor))
      ;;[1 1 1] If moving Up
      (if (> (.Z (Math|Vector|BreakVector (Transformation|GetVelocity _asaledgeclimbsystemcharacter_c))) 0.0)
        (if (Variables|Default|GetbCanGrabPressed _asaledgeclimbsystemcharacter_c)
          ;;[1 1 1] If pressing forward
          (if (Variables|Default|GetbMovingForward _asaledgeclimbsystemcharacter_c)
            ;;[1 1 1] Start to Climb Up the Ladder
            (Variables|Default|SetbTopGetOutTrigger false)
            (CallFunction|GetOutOfLadderTop _asaledgeclimbsystemcharacter_c)))))))

(event OnComponentEndOverlap(TopGetOutTrigger)
  (params (OverlappedComponent :type Primitive%20Component%20Object%20Reference) (OtherActor :type Actor%20Object%20Reference) (OtherComp :type Primitive%20Component%20Object%20Reference) (OtherBodyIndex :type Integer))
  ;[1 1 1] It just started to climb down the ladder
  (if (not (Variables|Default|GetbDisabled))
    (Variables|Default|SetbTopGetOutTrigger false)))

(event OnComponentBeginOverlap(TopClimbDownTrigger)
  (params (OverlappedComponent :type Primitive%20Component%20Object%20Reference) (OtherActor :type Actor%20Object%20Reference) (OtherComp :type Primitive%20Component%20Object%20Reference) (OtherBodyIndex :type Integer) (bFromSweep :type Boolean) (SweepResult :type Hit%20Result%20Structure%20%28by%20ref%29))
  ;[1 1 1] Show text when coming close to the top ladder, to climb down
  (if (not (Variables|Default|GetbDisabled))
    (Variables|Default|SetbTopClimbDownTrigger true)
    (if (not (Variables|Default|GetbTopGetOutTrigger))
      (bind _asaledgeclimbsystemcharacter_c (Utilities|Casting|CastTo OtherActor))
      ;;[1 1 1] If not moving up or downward
      (if (== (.Z (Math|Vector|BreakVector (Transformation|GetVelocity _asaledgeclimbsystemcharacter_c))) 0.0)
        (if (Variables|Default|GetbCanGrabPressed _asaledgeclimbsystemcharacter_c)
          (Variables|Default|SetbLadderTopVolume _asaledgeclimbsystemcharacter_c true)
          (Variables|Default|SetLadderToClimb _asaledgeclimbsystemcharacter_c self)
          (CallFunction|GetDownLadder _asaledgeclimbsystemcharacter_c))))))

(event OnComponentEndOverlap(LadderVolumeMesh)
  (params (OverlappedComponent :type Primitive%20Component%20Object%20Reference) (OtherActor :type Actor%20Object%20Reference) (OtherComp :type Primitive%20Component%20Object%20Reference) (OtherBodyIndex :type Integer))
  ;[1 1 1] Ladder In and Out
  (if (not (Variables|Default|GetbDisabled))
    (Variables|Default|SetbInLadderVolume false)
    (bind _asaledgeclimbsystemcharacter_c (Utilities|Casting|CastTo OtherActor))
    (Variables|Default|SetbInLadderVolume _asaledgeclimbsystemcharacter_c false)
    (Variables|Default|SetbLadderMoving _asaledgeclimbsystemcharacter_c false)
    (Variables|Default|SetbLadderTopVolume _asaledgeclimbsystemcharacter_c false)
    (Pawn|Components|CharacterMovement|SetMovementMode (Variables|/Script/Engine.Character|GetCharacterMovement _asaledgeclimbsystemcharacter_c) "MOVE_Walking" 0)))

(event OnComponentBeginOverlap(LadderOutTrigger)
  (params (OverlappedComponent :type Primitive%20Component%20Object%20Reference) (OtherActor :type Actor%20Object%20Reference) (OtherComp :type Primitive%20Component%20Object%20Reference) (OtherBodyIndex :type Integer) (bFromSweep :type Boolean) (SweepResult :type Hit%20Result%20Structure%20%28by%20ref%29))
  ;[1 1 1] Ladder outside in and out Trigger
  (Variables|Default|SetbLaddOutTrigger true)
  (bind _asaledgeclimbsystemcharacter_c (Utilities|Casting|CastTo OtherActor))
  (Variables|Default|SetbLadderOutTrigger _asaledgeclimbsystemcharacter_c true))

(event OnComponentEndOverlap(LadderOutTrigger)
  (params (OverlappedComponent :type Primitive%20Component%20Object%20Reference) (OtherActor :type Actor%20Object%20Reference) (OtherComp :type Primitive%20Component%20Object%20Reference) (OtherBodyIndex :type Integer))
  ;[1 1 1] Ladder outside in and out Trigger
  (Variables|Default|SetbLaddOutTrigger false)
  (bind _asaledgeclimbsystemcharacter_c (Utilities|Casting|CastTo OtherActor))
  (Variables|Default|SetbLadderOutTrigger _asaledgeclimbsystemcharacter_c false)
  ;;[1 1 1] Prevent the camera rotation from rotate the character on the ledge
  (Variables|/Script/Engine.Pawn|SetbUseControllerRotationYaw _asaledgeclimbsystemcharacter_c false)
  (Variables|/Script/Engine.CharacterMovementComponent|SetbOrientRotationToMovement (Variables|/Script/Engine.Character|GetCharacterMovement _asaledgeclimbsystemcharacter_c) true)
  (Variables|Default|SetbLadderFallingGrabbed _asaledgeclimbsystemcharacter_c false)
  (Variables|Default|SetbLadderStartToGetDown _asaledgeclimbsystemcharacter_c false))

(event EventBeginPlay
  ;[1 1 1] If the ladder is not configured right, it should be disabled in game
  (if (Rendering|IsVisible (Variables|Default|GetTextBadLadder))
    (Rendering|SetActorHiddenInGame true)
    (Collision|SetActorEnableCollision false)
    (Variables|Default|SetbDisabled true)))

(fn ConstructionScript
  (bind _textbadladder (Variables|Default|GetTextBadLadder))
  (bind _ladderouttrigger (Variables|Default|GetLadderOutTrigger))
  (bind _textclimbdown (Variables|Default|GetTextClimbDown))
  (bind _spherefortrace (Variables|Default|GetSphereForTrace))
  (bind _laddervolumemesh (Variables|Default|GetLadderVolumeMesh))
  (bind _arrow1 (Variables|Default|GetArrow1))
  (bind _topendmesh (Variables|Default|GetTopEndMesh))
  (bind _spherefortrace_2 (Variables|Default|GetSphereForTrace))
  (bind _topendmesh_2 (Variables|Default|GetTopEndMesh))
  (bind _textorientationhelper (Variables|Default|GetTextOrientationHelper))
  (bind _topendmesh_3 (Variables|Default|GetTopEndMesh))
  (bind _topclimbdowntrigger (Variables|Default|GetTopClimbDownTrigger))
  (bind _returnvalue (Transformation|GetWorldTransform _laddervolumemesh))
  (bind _returnvalue_2 (Transformation|GetWorldLocation _arrow1))
  (bind _returnvalue_3 (Transformation|GetWorldLocation _spherefortrace_2))
  (bind _returnvalue_4 (Transformation|GetWorldLocation _textorientationhelper))
  (bind _returnvalue_5 (Transformation|GetWorldLocation _spherefortrace))
  (bind _returnvalue_6 (Transformation|GetWorldLocation _textclimbdown))
  (bind _returnvalue_7 (Transformation|GetWorldTransform _ladderouttrigger))
  (bind _returnvalue_8 (Transformation|GetWorldLocation _topclimbdowntrigger))
  (bind _relativelocation (Variables|/Script/Engine.SceneComponent|GetRelativeLocation _topendmesh_2))
  (bind _relativelocation_2 (Variables|/Script/Engine.SceneComponent|GetRelativeLocation _textbadladder))
  (bind _relativelocation_3 (Variables|/Script/Engine.SceneComponent|GetRelativeLocation _topendmesh))
  (bind (_location _rotation _scale) (Math|Transform|BreakTransform _returnvalue))
  (bind (_x _y) (Math|Vector|BreakVector _returnvalue_2))
  (bind (_x_2 _y_2) (Math|Vector|BreakVector _returnvalue_3))
  (bind (_x_3 _y_3) (Math|Vector|BreakVector _relativelocation))
  (bind (_x_4 _y_4) (Math|Vector|BreakVector _relativelocation_3))
  (bind (_x_5 _y_5) (Math|Vector|BreakVector _relativelocation_2))
  (bind (_x_6 _y_6 _z) (Math|Vector|BreakVector _returnvalue_5))
  (bind (_x_7 _y_7) (Math|Vector|BreakVector _returnvalue_8))
  (bind (_x_8 _y_8) (Math|Vector|BreakVector _returnvalue_4))
  (bind (_x_9 _y_9) (Math|Vector|BreakVector _returnvalue_6))
  (bind (_location_2 _rotation_2 _scale_2) (Math|Transform|BreakTransform _returnvalue_7))
  (bind (_x_10 _y_10) (Math|Vector|BreakVector _scale))
  (bind (_x_11 _y_11) (Math|Vector|BreakVector _scale_2))
  (Transformation|SetActorRotation (Math|Rotator|MakeRotator 0.0 0.0 (.Yaw (Math|Rotator|BreakRotator (Transformation|GetActorRotation)))))
  (Components|StaticMesh|SetStaticMesh (Variables|ACLSLadder|GetLadder%20start) (Variables|Default|GetLadder%20Mesh)) ; Change spawned mesh to the new type
  (Variables|Default|SetLadder%20End (* (Variables|Default|GetLadder%20End) "0.000000,0.000000,1.000000"))
  (if (> (- (Math|Float|Round (/ (Math|Vector|VectorLength (* (Variables|Default|GetLadder%20End) "0.000000,0.000000,1.000000")) (Variables|Default|GetMesh%20width))) 1) 0) ; Don't spawn any meshes if none are needed
    (for _index (range 1 (- (Math|Float|Round (/ (Math|Vector|VectorLength (* (Variables|Default|GetLadder%20End) "0.000000,0.000000,1.000000")) (Variables|Default|GetMesh%20width))) 1)) ; Repeat once for every mesh to spawn
      (bind _returnvalue_9 (AddComponent|AddStaticMeshComponent true))
      (Class|SceneComponent|Attachto _returnvalue_9 (Variables|ACLSLadder|GetLadder%20start) "None" "KeepWorldPosition" true) ; Attach each segment to the initial mesh
      (Transformation|SetRelativeLocation _returnvalue_9 (Math|Vector|MakeVector 0.0 0.0 (* _index (Variables|Default|GetMesh%20width))) false false)
      (Components|StaticMesh|SetStaticMesh _returnvalue_9 (Variables|Default|GetLadder%20Mesh)) ; Change spawned mesh to the new type
      (Transformation|SetRelativeRotation _returnvalue_9 (Variables|/Script/Engine.SceneComponent|GetRelativeRotation (Variables|ACLSLadder|GetLadder%20start)) false false)
      (Transformation|SetWorldLocation _spherefortrace_2 (Math|Vector|MakeVector _x_2 _y_2 (+ (.Z (Math|Vector|BreakVector (Variables|Default|GetLadder%20End))) (.Z (Math|Vector|BreakVector (Transformation|GetActorLocation))))) false false)
      (Rendering|SetVisibility _returnvalue_9 true false)
      (Rendering|SetVisibility (Variables|ACLSLadder|GetLadder%20start) true false)
      (Rendering|SetVisibility _topendmesh_3 false false)
      (Components|StaticMesh|SetStaticMesh _topendmesh_3 (Variables|Default|GetLadder%20Top%20Mesh)) ; Change spawned mesh to the new type
      (Transformation|SetWorldTransform _laddervolumemesh (Math|Transform|MakeTransform _location _rotation (Math|Vector|MakeVector _x_10 _y_10 (+ (/ (Math|Vector|VectorLength (* (Variables|Default|GetLadder%20End) "0.000000,0.000000,1.000000")) (Variables|Default|GetMesh%20width)) 2.0))) true false)
      (Transformation|SetWorldTransform _ladderouttrigger (Math|Transform|MakeTransform _location_2 _rotation_2 (Math|Vector|MakeVector _x_11 _y_11 (Math|Conversions|ToFloat(Integer) (Math|Float|Round (/ (Math|Vector|VectorLength (* (Variables|Default|GetLadder%20End) "0.000000,0.000000,1.000000")) (Variables|Default|GetMesh%20width)))))) true false)
      (bind (_outhit _returnvalue_10) (Collision|LineTraceByChannel _returnvalue_5 (Math|Vector|MakeVector _x_6 _y_6 (- _z 5.0)) "TraceTypeQuery1" true 0 "None"))
      (if _returnvalue_10
        (Rendering|SetVisibility _textbadladder false false)
        (Transformation|SetWorldLocation _textorientationhelper (Math|Vector|MakeVector _x_8 _y_8 (.Z (Math|Vector|BreakVector (.ImpactPoint (Collision|BreakHitResult _outhit))))) false false)
        (Transformation|SetWorldLocation (Variables|Default|GetTopGetOutTrigger) (Math|Vector|MakeVector _x _y (+ (.Z (Math|Vector|BreakVector (.ImpactPoint (Collision|BreakHitResult _outhit)))) 4e+01)) false false)
        (Transformation|SetWorldLocation _topclimbdowntrigger (Math|Vector|MakeVector _x_7 _y_7 (+ (.Z (Math|Vector|BreakVector (.ImpactPoint (Collision|BreakHitResult _outhit)))) 3e+01)) false false)
        (Transformation|SetWorldLocation _textclimbdown (Math|Vector|MakeVector _x_9 _y_9 (+ (.Z (Math|Vector|BreakVector (.ImpactPoint (Collision|BreakHitResult _outhit)))) 1.3e+02)) false false)
        (Transformation|SetRelativeLocation _topendmesh (Math|Vector|MakeVector _x_4 _y_4 (- (.Z (Math|Vector|BreakVector (Variables|Default|GetLadder%20End))) 48.0)) false false)
        (Rendering|SetVisibility (Variables|Default|GetTopEndMesh) (Variables|Default|GetShowTopEndMesh) false)
        (else
          (Rendering|SetVisibility _textbadladder true false)
          (Transformation|SetRelativeLocation _textbadladder (Math|Vector|MakeVector _x_5 _y_5 (+ (.Z (Math|Vector|BreakVector (Variables|Default|GetLadder%20End))) 3e+01)) false false)
          (Transformation|SetRelativeLocation _topendmesh_2 (Math|Vector|MakeVector _x_3 _y_3 (- (.Z (Math|Vector|BreakVector (Variables|Default|GetLadder%20End))) 45.0)) false false)
          (Rendering|SetVisibility (Variables|Default|GetTopEndMesh) false false))))))