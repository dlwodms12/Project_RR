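; Climbable pole actor for a ledge climbing system, which tells the overlapping character when it can climb and where to stop.
; The Construction Script keeps the pole upright, stretches the hidden volume and optional visible mesh to the PoleEnd height, and places TopVolume there.
; When CanBeClimbed is set, volume overlaps set the character's pole-state flags, halting movement at the bottom or when rising into the top, and restoring walking on exit unless jumping back.
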(event OnComponentBeginOverlap(TopVolume)
  (params (OverlappedComponent :type Primitive%20Component%20Object%20Reference) (OtherActor :type Actor%20Object%20Reference) (OtherComp :type Primitive%20Component%20Object%20Reference) (OtherBodyIndex :type Integer) (bFromSweep :type Boolean) (SweepResult :type Hit%20Result%20Structure%20%28by%20ref%29))
  ;[1 1 1] Stop at the top, when touch the Top volume
  (if (Variables|Default|GetbCanBeClimbed)
    (bind _asaledgeclimbsystemcharacter_c (Utilities|Casting|CastTo OtherActor))
    (if (> (.Z (Math|Vector|BreakVector (Transformation|GetVelocity _asaledgeclimbsystemcharacter_c))) 0.0)
      (Components|Movement|StopMovementImmediately (Variables|/Script/Engine.Character|GetCharacterMovement _asaledgeclimbsystemcharacter_c))
      (Variables|Default|SetbStopMovement _asaledgeclimbsystemcharacter_c true)
      (Variables|Default|SetbPoleTopVolume _asaledgeclimbsystemcharacter_c true))))

(event OnComponentEndOverlap(TopVolume)
  (params (OverlappedComponent :type Primitive%20Component%20Object%20Reference) (OtherActor :type Actor%20Object%20Reference) (OtherComp :type Primitive%20Component%20Object%20Reference) (OtherBodyIndex :type Integer))
  ;[1 1 1] Stop at the top, when touch the Top volume
  (if (Variables|Default|GetbCanBeClimbed)
    (bind _asaledgeclimbsystemcharacter_c (Utilities|Casting|CastTo OtherActor))
    (Variables|Default|SetbPoleTopVolume _asaledgeclimbsystemcharacter_c false)))

(event OnComponentBeginOverlap(PoleVolumeMesh)
  (params (OverlappedComponent :type Primitive%20Component%20Object%20Reference) (OtherActor :type Actor%20Object%20Reference) (OtherComp :type Primitive%20Component%20Object%20Reference) (OtherBodyIndex :type Integer) (bFromSweep :type Boolean) (SweepResult :type Hit%20Result%20Structure%20%28by%20ref%29))
  ;[1 1 1] Enter or get out of Pole Volume
  (if (Variables|Default|GetbCanBeClimbed)
    (bind _asaledgeclimbsystemcharacter_c (Utilities|Casting|CastTo OtherActor))
    (Variables|Default|SetbInPoleVolume _asaledgeclimbsystemcharacter_c true)
    (Variables|Default|SetPoleToClimb _asaledgeclimbsystemcharacter_c self)
    (Variables|Default|SetbPolePositioned _asaledgeclimbsystemcharacter_c false)))

(event OnComponentBeginOverlap(BottomVolume)
  (params (OverlappedComponent :type Primitive%20Component%20Object%20Reference) (OtherActor :type Actor%20Object%20Reference) (OtherComp :type Primitive%20Component%20Object%20Reference) (OtherBodyIndex :type Integer) (bFromSweep :type Boolean) (SweepResult :type Hit%20Result%20Structure%20%28by%20ref%29))
  ;[1 1 1] Stop at the bottom, when touch at the bottom volume
  (if (Variables|Default|GetbCanBeClimbed)
    (bind _asaledgeclimbsystemcharacter_c (Utilities|Casting|CastTo OtherActor))
    (Components|Movement|StopMovementImmediately (Variables|/Script/Engine.Character|GetCharacterMovement _asaledgeclimbsystemcharacter_c))
    (Variables|Default|SetbStopMovement _asaledgeclimbsystemcharacter_c true)
    (Variables|Default|SetbPoleBottomVolume _asaledgeclimbsystemcharacter_c true)))

(event OnComponentEndOverlap(PoleVolumeMesh)
  (params (OverlappedComponent :type Primitive%20Component%20Object%20Reference) (OtherActor :type Actor%20Object%20Reference) (OtherComp :type Primitive%20Component%20Object%20Reference) (OtherBodyIndex :type Integer))
  ;[1 1 1] Enter or get out of Pole Volume
  (if (Variables|Default|GetbCanBeClimbed)
    (bind _asaledgeclimbsystemcharacter_c (Utilities|Casting|CastTo OtherActor))
    (Variables|Default|SetbInPoleVolume _asaledgeclimbsystemcharacter_c false)
    (Variables|Default|SetbPoleMoving _asaledgeclimbsystemcharacter_c false)
    (Variables|Default|SetbPolePositioned _asaledgeclimbsystemcharacter_c false)
    (Variables|Default|SetbPoleStarttoGetDown _asaledgeclimbsystemcharacter_c false)
    (Variables|Default|SetbPoleFallingGrabbed _asaledgeclimbsystemcharacter_c false)
    (if (not (Variables|Default|GetbJumpingBack _asaledgeclimbsystemcharacter_c))
      (Pawn|Components|CharacterMovement|SetMovementMode (Variables|/Script/Engine.Character|GetCharacterMovement _asaledgeclimbsystemcharacter_c) "MOVE_Walking" 0))))

(event OnComponentEndOverlap(BottomVolume)
  (params (OverlappedComponent :type Primitive%20Component%20Object%20Reference) (OtherActor :type Actor%20Object%20Reference) (OtherComp :type Primitive%20Component%20Object%20Reference) (OtherBodyIndex :type Integer))
  ;[1 1 1] Stop at the bottom, when touch at the bottom volume
  (if (Variables|Default|GetbCanBeClimbed)
    (bind _asaledgeclimbsystemcharacter_c (Utilities|Casting|CastTo OtherActor))
    (Variables|Default|SetbPoleBottomVolume _asaledgeclimbsystemcharacter_c false)))

(fn ConstructionScript
  (bind _polevolumemesh (Variables|Default|GetPoleVolumeMesh))
  (bind _polemeshcomp (Variables|Default|GetPoleMeshComp))
  (bind _fdivisor (Variables|Default|GetfDivisor))
  (bind _returnvalue (Transformation|GetWorldTransform _polevolumemesh))
  (bind _returnvalue_2 (Transformation|GetWorldTransform _polemeshcomp))
  (bind (_location _rotation _scale) (Math|Transform|BreakTransform _returnvalue))
  (bind (_location_2 _rotation_2 _scale_2) (Math|Transform|BreakTransform _returnvalue_2))
  (bind (_x _y) (Math|Vector|BreakVector _scale))
  (bind (_x_2 _y_2) (Math|Vector|BreakVector _scale_2))
  (Transformation|SetActorRotation (Math|Rotator|MakeRotator 0.0 0.0 (.Yaw (Math|Rotator|BreakRotator (Transformation|GetActorRotation)))))
  (Variables|Default|SetPole%20End (* (Variables|Default|GetPole%20End) "0.000000,0.000000,1.000000"))
  (Rendering|SetVisibility (Variables|Default|GetPoleVolumeMesh) false false)
  (Transformation|SetWorldTransform _polevolumemesh (Math|Transform|MakeTransform _location _rotation (Math|Vector|MakeVector _x _y (/ (Math|Vector|VectorLength (* (Variables|Default|GetPole%20End) "0.000000,0.000000,1.000000")) (Variables|Default|GetMesh%20width)))) true false)
  (Rendering|SetVisibility (Variables|Default|GetPoleMeshComp) (Variables|Default|GetShowPole) false)
  (Transformation|SetWorldTransform _polemeshcomp (Math|Transform|MakeTransform _location_2 _rotation_2 (Math|Vector|MakeVector (/ _x_2 _fdivisor) (/ _y_2 _fdivisor) (/ (Math|Vector|VectorLength (* (Variables|Default|GetPole%20End) "0.000000,0.000000,1.000000")) (Variables|Default|GetMesh%20width)))) true false)
  (Transformation|SetRelativeLocation (Variables|Default|GetTopVolume) (Math|Vector|MakeVector (.X (Math|Vector|BreakVector (Variables|Default|GetPole%20End))) (.Y (Math|Vector|BreakVector (Variables|Default|GetPole%20End))) (.Z (Math|Vector|BreakVector (Variables|Default|GetPole%20End)))) false false))