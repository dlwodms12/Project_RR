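; Climbable ladder zone for the custom movement system, registering itself with BP_CustomMoveThirdPersonCharacter while that character overlaps its trigger box.
; The Construction Script builds cube rungs from StepCount and StepHeight, stretches the trigger, and offsets Top and TopEnter relative to a four-step baseline.
; Query functions test character bottom position and input for entering at bottom, middle or top and exiting at either end.
; Getters expose ladder endpoints, rotation, step height and top-entry location.
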(event OnComponentBeginOverlap(TriggerBox)
  (params (OverlappedComponent :type Primitive%20Component%20Object%20Reference) (OtherActor :type Actor%20Object%20Reference) (OtherComp :type Primitive%20Component%20Object%20Reference) (OtherBodyIndex :type Integer) (bFromSweep :type Boolean) (SweepResult :type Hit%20Result%20Structure%20%28by%20ref%29))
  (bind _asbp_custom_move_third_person_character (Utilities|Casting|CastToBP_CustomMoveThirdPersonCharacter OtherActor))
  (Default|BeginOverlappedCustomMoveZone _asbp_custom_move_third_person_character (Utilities|Struct|MakeSCustomMoveZone self "NewEnumerator0")))

(event OnComponentEndOverlap(TriggerBox)
  (params (OverlappedComponent :type Primitive%20Component%20Object%20Reference) (OtherActor :type Actor%20Object%20Reference) (OtherComp :type Primitive%20Component%20Object%20Reference) (OtherBodyIndex :type Integer))
  (bind _asbp_custom_move_third_person_character (Utilities|Casting|CastToBP_CustomMoveThirdPersonCharacter OtherActor))
  (Default|EndOverlappedCustomMoveZone _asbp_custom_move_third_person_character self))

(event EventBeginPlay)

(event Collision|EventActorBeginOverlap
  (params (OtherActor :type Actor%20Object%20Reference)))

(event EventTick
  (params (DeltaSeconds :type Float%20%28single-precision%29)))

(fn ConstructionScript
  (bind _step_count (Variables|Ladder|GetStep%20Count))
  (bind _step_count_2 (Variables|Ladder|GetStep%20Count))
  (bind _triggerbox (Variables|Default|GetTriggerBox))
  (bind _triggerbox_2 (Variables|Default|GetTriggerBox))
  (bind _step_height (Variables|Ladder|GetStep%20Height))
  (bind _top (Variables|Default|GetTop))
  (bind _top_enter (Variables|Default|GetTop_Enter))
  (bind _returnvalue (- _step_count_2 4))
  (bind _returnvalue_2 (Math|Conversions|ToFloat(Integer) _step_count))
  (bind _relativescale3d (Variables|/Script/Engine.SceneComponent|GetRelativeScale3D _triggerbox))
  (bind _relativelocation (Variables|/Script/Engine.SceneComponent|GetRelativeLocation _triggerbox_2))
  (bind _relativelocation_2 (Variables|/Script/Engine.SceneComponent|GetRelativeLocation _top_enter))
  (bind _relativelocation_3 (Variables|/Script/Engine.SceneComponent|GetRelativeLocation _top))
  (bind _returnvalue_3 (* _returnvalue _step_height))
  (bind _returnvalue_4 (/ _returnvalue_2 4.0))
  (Transformation|SetRelativeScale3D _triggerbox (Math|Vector|MakeVector (.x _relativescale3d) (.y _relativescale3d) (* (+ (.z _relativescale3d) (/ 0.5 _returnvalue_4)) _returnvalue_4)))
  (Transformation|SetRelativeLocation _triggerbox_2 (Math|Vector|MakeVector (.x _relativelocation) (.y _relativelocation) (.Z (Math|Vector|BreakVector (.BoxExtent (Collision|GetComponentBounds _triggerbox_2))))) false false)
  (Transformation|SetRelativeLocation _top (Math|Vector|MakeVector (.x _relativelocation_3) (.y _relativelocation_3) (+ (.z _relativelocation_3) _returnvalue_3)) false false)
  (Transformation|SetRelativeLocation _top_enter (Math|Vector|MakeVector (.x _relativelocation_2) (.y _relativelocation_2) (+ (.z _relativelocation_2) _returnvalue_3)) false false)
  (for _index (range 1 (Variables|Ladder|GetStep%20Count))
    (bind _returnvalue_5 (AddComponent|AddStaticMeshComponent false (Math|Transform|MakeTransform (Math|Vector|MakeVector 0.0 0.0 (* _index (Variables|Ladder|GetStep%20Height))) "0, 0, 0" "0.100000,1.000000,0.100000")))
    (Components|StaticMesh|SetStaticMesh _returnvalue_5 "/Game/11_CustomMovement/Meshes/SM_Cube.SM_Cube")))

(fn CheckEntertoBottom
  (params (Character%20Bottom%20Location :type Vector :default "0, 0, 0") (Input%20Direction :type Vector :default "0, 0, 0") (Input%20Scale :type Float%20%28double-precision%29))
  (bind _returnvalue (Transformation|GetActorForwardVector))
  (return (and (<= (Math|Vector|VectorLength (- Character%20Bottom%20Location (Transformation|GetWorldLocation (Variables|Default|GetBottom)))) 5e+01) (or (and (> Input%20Scale 0.8) (>= (Math|Vector|DotProduct Input%20Direction _returnvalue) 0.7)) (and (<= (Math|Vector|DotProduct _returnvalue Input%20Direction) -0.7) (< Input%20Scale -0.8))))))

(fn CheckEntertoMiddle
  (params (Character%20Bottom%20Location :type Vector :default "0, 0, 0") (Input%20Direction :type Vector :default "0, 0, 0") (Input%20Scale :type Float%20%28double-precision%29))
  (bind _returnvalue (Transformation|GetActorForwardVector))
  (return (and (> (Math|Vector|VectorLength (- Character%20Bottom%20Location (Transformation|GetWorldLocation (Variables|Default|GetBottom)))) 5e+01) (or (and (> Input%20Scale 0.8) (>= (Math|Vector|DotProduct Input%20Direction _returnvalue) 0.7)) (and (<= (Math|Vector|DotProduct _returnvalue Input%20Direction) -0.7) (< Input%20Scale -0.8))))))

(fn CheckEntertoTop
  (params (Character%20Bottom%20Location :type Vector :default "0, 0, 0") (Input%20Direction :type Vector :default "0, 0, 0") (Input%20Scale :type Float%20%28double-precision%29))
  (bind _returnvalue (Transformation|GetActorForwardVector))
  (return (and (<= (Math|Vector|VectorLength (- Character%20Bottom%20Location (Transformation|GetWorldLocation (Variables|Default|GetTop_Enter)))) 5e+01) (or (and (> Input%20Scale 0.3) (<= (Math|Vector|DotProduct Input%20Direction _returnvalue) -0.7)) (and (>= (Math|Vector|DotProduct _returnvalue Input%20Direction) 0.7) (< Input%20Scale -0.3))))))

(fn CheckExittoBottom
  (params (Character%20Bottom%20Location :type Vector :default "0, 0, 0") (Input%20Scale :type Float%20%28double-precision%29))
  (return (and (< Input%20Scale -0.8) (<= (Math|Vector|VectorLength (- Character%20Bottom%20Location (Transformation|GetWorldLocation (Variables|Default|GetBottom)))) 1.0))))

(fn CheckExittoTop
  (params (Character%20Bottom%20Location :type Vector :default "0, 0, 0") (Input%20Scale :type Float%20%28double-precision%29))
  (return (and (> Input%20Scale 0.8) (<= (Math|Vector|VectorLength (- Character%20Bottom%20Location (Transformation|GetWorldLocation (Variables|Default|GetTop)))) 1.0))))

(fn GetLadderLocation
  (return (Transformation|GetWorldLocation (Variables|Default|GetTop)) (Transformation|GetWorldLocation (Variables|Default|GetBottom))))

(fn GetLadderRotation
  (return (Transformation|GetActorRotation)))

(fn GetLadderStepHeight
  (return (Variables|Ladder|GetStep%20Height)))

(fn GetTopEnterLocation
  (return (Transformation|GetWorldLocation (Variables|Default|GetTop_Enter))))