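; BP_Test is an actor that makes its static mesh bob vertically and spin around yaw, apparently as a test asset.
; Tick accumulates delta time in Location, adds its sine to the mesh's current world Z and sets an absolute yaw proportional to that time.
; The sine offset compounds every frame, so bob height depends on frame rate.
; An actor rotation node is left unconnected, and no replication logic appears in the graphs.
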(event EventBeginPlay)

(event Collision|EventActorBeginOverlap
  (params (OtherActor :type Actor%20Object%20Reference)))

(event EventTick
  (params (DeltaSeconds :type Float%20%28single-precision%29))
  (bind _staticmesh (Variables|Default|GetStaticMesh))
  (bind _returnvalue (Transformation|GetWorldLocation _staticmesh))
  (bind (_x _y _z) (Math|Vector|BreakVector _returnvalue))
  (bind _output_get (Variables|Default|SetLocation (+ DeltaSeconds (Variables|Default|GetLocation))))
  (bind _output_get_2 (Variables|Default|SetNewLocation (Math|Vector|MakeVector _x _y (+ (Math|Trig|Sin(Radians) _output_get) _z))))
  (Transformation|SetWorldLocationAndRotation (Variables|Default|GetStaticMesh) _output_get_2 (Math|Rotator|MakeRotator 0.0 0.0 (* (Variables|Default|GetLocation) 15.0)) false false))

(fn ConstructionScript)