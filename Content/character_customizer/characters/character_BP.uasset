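; Playable third-person character for the character customizer, with yaw-relative movement, jump, slow walk and smoothly interpolated mouse-wheel zoom.
; It caches its Character_customizer component, whose menu a custom event toggles.
; Tab line-traces from the camera to possess another character_BP, closing the menu first.
; A randomized timeline drives eye-blink morph targets; camera FOV, mode and offset graphs are unwired.
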(event Custom|menu%20toggle%20button
  ;[1 1 1] character customizer
  ;;[1 1 1] toggle character customizer
  (Default|MenuToggle (Variables|Default|Getcharacter_customizer)))

(event Custom|Blink_event
  (bind _mesh (Variables|Character|GetMesh))
  ;[1 1 1] character customizer
  ;;[1 1 1] blink
  (bind _blink (Timeline|Blinking PlayFromStart)
    (:Update
      (Components|Timeline|SetPlayRate (Variables|Default|Getblinking) (Math|Random|RandomFloatinRange 0.2 1.5))
      (Components|SkeletalMesh|SetMorphTarget _mesh "eyes_closed_left" _blink true)
      (Components|SkeletalMesh|SetMorphTarget _mesh "eyes_closed_right" _blink true)
      (Utilities|FlowControl|Delay (Math|Random|RandomFloatinRange 0.5 8.0))
      (CallFunction|BlinkEvent))))

(event EventBeginPlay
  ;[1 1 1] beginplay
  (Utilities|FlowControl|Sequence
    (:then_0
      (CallFunction|BlinkEvent))
    (:then_1
      (Variables|Default|Setcharacter_customizer (Actor|GetComponentbyClass "/Game/character_customizer/project_files/character_customizer.character_customizer_C")))))

(event EventTick
  (params (DeltaSeconds :type Float%20%28single-precision%29))
  ;[1 1 1] tick
  ;[1 1 1] camera
  ;;[1 1 1] zoom
  (Variables|/Script/Engine.SpringArmComponent|SetTargetArmLength (Variables|Default|GetSpringArm) (Math|Interpolation|FInterpTo (Variables|/Script/Engine.SpringArmComponent|GetTargetArmLength (Variables|Default|GetSpringArm)) (Variables|Camera|Getcamera%20arm%20length) (Utilities|Time|GetWorldDeltaSeconds) 5.0)))

(event Input|ActionEvents|InputActionJump
  (params (Key :type Key%20Structure :default "None"))
  ;[1 1 1] movement
  (:Pressed
    (Character|Jump)))

(event Input|AxisEvents|InputAxisTurn
  (params (AxisValue :type Float%20%28single-precision%29))
  ;[1 1 1] movement
  (Pawn|Input|AddControllerYawInput AxisValue))

(event Input|AxisEvents|InputAxisLookUp
  (params (AxisValue :type Float%20%28single-precision%29))
  ;[1 1 1] movement
  (Pawn|Input|AddControllerPitchInput AxisValue))

(event Input|AxisEvents|InputAxisMoveRight
  (params (AxisValue :type Float%20%28single-precision%29))
  ;[1 1 1] movement
  (Pawn|Input|AddMovementInput (Math|Vector|GetRightVector (Math|Rotator|MakeRotator 0.0 0.0 (.Yaw (Math|Rotator|BreakRotator (Pawn|GetControlRotation :!class /Script/Engine.Pawn))))) AxisValue false))

(event Input|AxisEvents|InputAxisMoveForward
  (params (AxisValue :type Float%20%28single-precision%29))
  ;[1 1 1] movement
  (Pawn|Input|AddMovementInput (Math|Vector|GetForwardVector (Math|Rotator|MakeRotator 0.0 0.0 (.Yaw (Math|Rotator|BreakRotator (Pawn|GetControlRotation :!class /Script/Engine.Pawn))))) AxisValue false))

(event Input|KeyboardEvents|Tab
  (params (Key :type Key%20Structure :default "None"))
  ;[1 1 1] character customizer
  ;;[1 1 1] possess
  (:Pressed
    (CallFunction|Possess)))

(event Input|KeyboardEvents|LeftCtrl
  (params (Key :type Key%20Structure :default "None"))
  (bind _charactermovement (Variables|Character|GetCharacterMovement))
  ;[1 1 1] movement
  (:Pressed
    (Variables|/Script/Engine.CharacterMovementComponent|SetMaxWalkSpeed _charactermovement 135.0))
  (:Released
    (Variables|/Script/Engine.CharacterMovementComponent|SetMaxWalkSpeed _charactermovement 3.6e+02)))

(event Input|MouseEvents|MouseWheelDown
  (params (Key :type Key%20Structure :default "None"))
  ;[1 1 1] camera
  ;;[1 1 1] zoom
  (:Pressed
    (Variables|Camera|Setcamera%20arm%20length (+ (Variables|Camera|Getcamera%20arm%20length) (Variables|Camera|Getzoom%20amount)))))

(event Input|MouseEvents|MouseWheelUp
  (params (Key :type Key%20Structure :default "None"))
  ;[1 1 1] camera
  ;;[1 1 1] zoom
  (:Pressed
    (Variables|Camera|Setcamera%20arm%20length (- (Variables|Camera|Getcamera%20arm%20length) (Variables|Camera|Getzoom%20amount)))))

(fn ConstructionScript)

(fn Possess
  (bind _returnvalue (Game|GetPlayerController 0))
  (bind _returnvalue_2 (Game|GetPlayerCameraManager 0))
  (bind _returnvalue_3 (Camera|GetCameraLocation _returnvalue_2))
  (bind (_outhit _returnvalue_4) (Collision|LineTraceForObjects _returnvalue_3 (+ _returnvalue_3 (* (Transformation|GetActorForwardVector _returnvalue_2) 1e+04)) (Utilities|Array|MakeArray "ObjectTypeQuery3") false 0 "None"))
  (if _returnvalue_4
    (bind _ascharacter_bp (Utilities|Casting|CastTocharacter_BP (.hitactor _outhit)))
    (Default|MenuExit (Variables|Default|Getcharacter_customizer))
    (Pawn|UnPossess _returnvalue)
    (Pawn|Possess _returnvalue _ascharacter_bp)))