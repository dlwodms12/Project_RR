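; Space pawn child Blueprint that adds thruster particle effects and a toggleable flashlight.
; After the parent Tick, it feeds the inverted ThrustVector into the particle system's Thrust vector parameter.
; The C key calls FlashLight, which relays to FlashLightMulti to toggle the spotlight by subtracting its current intensity from a fixed value.
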(event Custom|FlashLight
  (CallFunction|FlashLightMulti))

(event Custom|FlashLightMulti
  (bind _spotlight (Variables|Default|GetSpotLight))
  (Rendering|Components|Light|SetIntensity _spotlight (- 2.5e+02 (Variables|/Script/Engine.LightComponentBase|GetIntensity _spotlight))))

(event EventBeginPlay)

(event Collision|EventActorBeginOverlap
  (params (OtherActor :type Actor%20Object%20Reference)))

(event EventTick
  (params (DeltaSeconds :type Float%20%28single-precision%29))
  (|CallParentFunction DeltaSeconds)
  (Effects|Components|ParticleSystem|SetVectorParameter (Variables|Default|GetParticleSystem) "Thrust" (* (Variables|Default|GetThrustVector) -1.0)))

(event Input|KeyboardEvents|C
  (params (Key :type Key%20Structure))
  (:Pressed
    (CallFunction|FlashLight)))

(fn ConstructionScript
  (|CallParentFunction))