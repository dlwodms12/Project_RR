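; BP_Door is an interactable sliding double door with two mesh halves that open and close in opposite directions.
; An Interact hit on its Box component calls M_ToggleDoor, which flips the DoorState flag.
; Tick moves a clamped offset at constant speed toward the limit selected by that flag and applies it, mirrored, to both halves' relative Y positions without sweeping.
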(event Custom|M_ToggleDoor
  (Variables|Default|SetDoorState (not (Variables|Default|GetDoorState))))

(event EventTick
  (params (DeltaSeconds :type Float%20%28single-precision%29))
  (bind _output_get (Variables|Default|SetDoorOffset (Math|Float|Clamp(Float) (+ (Variables|Default|GetDoorOffset) (* DeltaSeconds (Math|Float|SelectFloat 1e+02 -1e+02 (Variables|Default|GetDoorState)))) 75.0 175.0)))
  (Transformation|SetRelativeLocation (Variables|Default|GetCube1) (Math|Vector|MakeVector 0.0 (* _output_get -1.0) 0.0) false false)
  (Transformation|SetRelativeLocation (Variables|Default|GetStaticMesh1) (Math|Vector|MakeVector 0.0 _output_get 0.0) false false))

(event EventInteract
  (params (Pawn :type BP%20Space%20Pawn%20Object%20Reference) (Hit :type Hit%20Result%20Structure))
  (if (== (Variables|Default|GetBox) (.HitComponent (Collision|BreakHitResult Hit)))
    (CallFunction|MToggleDoor)))

(fn ConstructionScript)