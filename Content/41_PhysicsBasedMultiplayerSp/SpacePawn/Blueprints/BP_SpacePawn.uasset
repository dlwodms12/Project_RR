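; Multiplayer space pawn flown with physics-based six-axis thrust and rotation, with switchable first/third-person zoom camera and trace-based interaction.
; Client inputs go to server events that set thrust and rotation vectors, which Tick applies as capsule impulses and torques.
; An optional stabilizer toggles linear and angular damping, normally when input is idle.
; The authority feeds its transform each tick into a lerped physics correction for replication.
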(event Custom|CameraTick
  (bind _springarm (Variables|Default|GetSpringArm))
  ;[1 1 1] CameraTick
  (Variables|/Script/Engine.SpringArmComponent|SetTargetArmLength _springarm (Math|Float|Lerp (Variables|/Script/Engine.SpringArmComponent|GetTargetArmLength _springarm) (Variables|Camera|GetTargetDistance) (* (Utilities|Time|GetWorldDeltaSeconds) (Variables|Camera|GetCameraChangeSpeed))))
  (Variables|/Script/Engine.SpringArmComponent|SetSocketOffset _springarm (Math|Vector|Lerp(Vector) (Variables|/Script/Engine.SpringArmComponent|GetSocketOffset _springarm) (Variables|Camera|GetTargetOffset) (* (Utilities|Time|GetWorldDeltaSeconds) (Variables|Camera|GetCameraChangeSpeed)))))

(event Custom|S_Stabilizer
  ;[1 1 1] Stabilizer on/off
  (Variables|Default|SetenableStabilizer (not (Variables|Default|GetenableStabilizer))))

(event Custom|S_MoveForward
  (params (Axis :type Float%20%28single-precision%29))
  ;[1 1 1] Forward
  (Variables|Default|SetThrustVector (Math|Vector|MakeVector Axis (.Y (Math|Vector|BreakVector (Variables|Default|GetThrustVector))) (.Z (Math|Vector|BreakVector (Variables|Default|GetThrustVector))))))

(event Custom|MovementStabilizerTick
  ;[1 1 1] MovementStabilizer
  (Class|PrimitiveComponent|SetLinearDamping (Variables|Default|GetCapsule) (Math|Float|SelectFloat (Variables|Stabilizer|GetMovementStabilizerMultiplier) 0.0 (and (Variables|Default|GetenableStabilizer) (or (Variables|Stabilizer|GetalwaysStabilize) (Math|Float|NearlyEqual(Float) (Math|Vector|VectorLength (Variables|Default|GetThrustVector)) 0.0 0.1))))))

(event Custom|S_MoveRight
  (params (Axis :type Float%20%28single-precision%29))
  ;[1 1 1] Right
  (Variables|Default|SetThrustVector (Math|Vector|MakeVector (.X (Math|Vector|BreakVector (Variables|Default|GetThrustVector))) Axis (.Z (Math|Vector|BreakVector (Variables|Default|GetThrustVector))))))

(event Custom|RotationTick
  (params (Delta :type Float%20%28single-precision%29))
  (bind _rotvector (Variables|Default|GetRotVector))
  (bind (_x _y _z) (Math|Vector|BreakVector _rotvector))
  ;[1 1 1] Rotation Tick
  (Class|PrimitiveComponent|AddTorqueinDegrees (Variables|Default|GetCapsule) (* (+ (* (Transformation|GetActorForwardVector) _x) (* (Transformation|GetActorRightVector) _y) (* (Transformation|GetActorUpVector) _z)) (* Delta (Variables|Thrust|GetRotMultiplier))) "None" true))

(event Custom|S_RotRoll
  (params (Axis :type Float%20%28single-precision%29))
  ;[1 1 1] Roll
  (Variables|Default|SetRotVector (Math|Vector|MakeVector Axis (.Y (Math|Vector|BreakVector (Variables|Default|GetRotVector))) (.Z (Math|Vector|BreakVector (Variables|Default|GetRotVector))))))

(event Custom|S_RotYaw
  (params (Axis :type Float%20%28single-precision%29))
  ;[1 1 1] Yaw
  (Variables|Default|SetRotVector (Math|Vector|MakeVector (.X (Math|Vector|BreakVector (Variables|Default|GetRotVector))) (.Y (Math|Vector|BreakVector (Variables|Default|GetRotVector))) Axis)))

(event Custom|S_RotPitch
  (params (Axis :type Float%20%28single-precision%29))
  ;[1 1 1] Pitch
  (Variables|Default|SetRotVector (Math|Vector|MakeVector (.X (Math|Vector|BreakVector (Variables|Default|GetRotVector))) Axis (.Z (Math|Vector|BreakVector (Variables|Default|GetRotVector))))))

(event Custom|S_MoveUp
  (params (Axis :type Float%20%28single-precision%29))
  ;[1 1 1] Up
  (Variables|Default|SetThrustVector (Math|Vector|MakeVector (.X (Math|Vector|BreakVector (Variables|Default|GetThrustVector))) (.Y (Math|Vector|BreakVector (Variables|Default|GetThrustVector))) Axis)))

(event Custom|RotationStabilizerTick
  ;[1 1 1] MovementStabilizer
  (Class|PrimitiveComponent|SetAngularDamping (Variables|Default|GetCapsule) (Math|Float|SelectFloat (Variables|Stabilizer|GetRotationStabilizerMultiplier) 0.0 (and (Variables|Default|GetenableStabilizer) (or (Variables|Stabilizer|GetalwaysStabilize) (Math|Float|NearlyEqual(Float) (Math|Vector|VectorLength (Variables|Default|GetRotVector)) 0.0 0.1))))))

(event Custom|S_Interact
  (params (Target :type Object%20Object%20Reference) (Hit :type Hit%20Result%20Structure))
  ;[1 1 1] Server Interact
  (Class|BIInteract|Interact(Message) Target self Hit))

(event Custom|MovementTick
  (params (Delta :type Float%20%28single-precision%29))
  (bind _thrustvector (Variables|Default|GetThrustVector))
  (bind (_x _y _z) (Math|Vector|BreakVector _thrustvector))
  ;[1 1 1] Movement Tick
  (Physics|AddImpulse (Variables|Default|GetCapsule) (* (+ (* (Transformation|GetActorForwardVector) _x) (* (Transformation|GetActorRightVector) _y) (* (Transformation|GetActorUpVector) _z)) (* Delta (Variables|Thrust|GetThrustMultiplier))) "None" true))

(event Custom|PhysicsCorrection
  (params (Pos :type Vector) (Rot :type Rotator))
  (bind _returnvalue (Utilities|Time|GetWorldDeltaSeconds))
  ;[1 1 1] Physics Correction (Replication)
  (Transformation|SetActorLocationAndRotation (Math|Vector|Lerp(Vector) Pos (Transformation|GetActorLocation) _returnvalue) (Math|Rotator|Lerp(Rotator) Rot (Transformation|GetActorRotation) _returnvalue true)))

(event EventTick
  (params (DeltaSeconds :type Float%20%28single-precision%29))
  ;[1 1 1] Tick
  (Utilities|FlowControl|Sequence
    (:then_0
      (CallFunction|MovementStabilizerTick)
      (CallFunction|MovementTick DeltaSeconds)
      (CallFunction|RotationStabilizerTick)
      (CallFunction|RotationTick DeltaSeconds)
      (CallFunction|CameraTick))
    (:then_1
      (Networking|SwitchHasAuthority
        (:Authority
          (CallFunction|PhysicsCorrection (Transformation|GetActorLocation) (Transformation|GetActorRotation)))))))

(event Input|ActionEvents|InputActionSwitchCamera
  (params (Key :type Key%20Structure))
  ;[1 1 1] Camera
  (:Pressed
    (Utilities|FlowControl|FlipFlop
      (:A
        (Variables|Camera|SetTargetDistance 0.0)
        (Variables|Camera|SetTargetOffset "0, 0, 0"))
      (:B
        (Variables|Camera|SetTargetDistance (Variables|Camera|GetCameraDistance))
        (Variables|Camera|SetTargetOffset (Variables|Camera|GetThirdpersonOffset))))))

(event Input|ActionEvents|InputActionInteract
  (params (Key :type Key%20Structure))
  (bind _camera (Variables|Default|GetCamera))
  (bind _returnvalue (Transformation|GetWorldLocation _camera))
  ;[1 1 1] Interact
  (:Pressed
    (bind _outhits (Collision|MultiLineTraceByChannel _returnvalue (+ _returnvalue (* (Math|Rotator|GetRotationXVector (Transformation|GetWorldRotation _camera)) (+ (Variables|Camera|GetTargetDistance) (Variables|Interact|GetInteractDistance)))) "TraceTypeQuery1" false 0 "None"))
    (bind (_closest _hit) (CallFunction|GetClosestInteractable _outhits))
    (CallFunction|SInteract _closest _hit)))

(event Input|ActionEvents|InputActionStabilizer
  (params (Key :type Key%20Structure))
  ;[1 1 1] Client Stabilizer
  (:Pressed
    (CallFunction|SStabilizer)))

(event Input|AxisEvents|InputAxisZoom
  (params (AxisValue :type Float%20%28single-precision%29))
  ;[1 1 1] Zoom
  (if (Variables|Camera|GetenableZoom)
    (if (and (!= (Variables|Camera|GetTargetDistance) 0.0) (!= AxisValue 0.0))
      (bind _output_get (Variables|Camera|SetCameraDistance (Math|Float|Clamp(Float) (+ (* AxisValue (Variables|Camera|GetZoomSpeed)) (Variables|Camera|GetCameraDistance)) (Variables|Camera|GetZoomMinDistance) (Variables|Camera|GetZoomMaxDistance))))
      (Variables|Camera|SetTargetDistance _output_get))))

(event Input|AxisEvents|InputAxisMoveForward
  (params (AxisValue :type Float%20%28single-precision%29))
  ;[1 1 1] Client Movement Inputs
  (CallFunction|SMoveForward AxisValue))

(event Input|AxisEvents|InputAxisMoveRight
  (params (AxisValue :type Float%20%28single-precision%29))
  ;[1 1 1] Client Movement Inputs
  (CallFunction|SMoveRight AxisValue))

(event Input|AxisEvents|InputAxisMoveUp
  (params (AxisValue :type Float%20%28single-precision%29))
  ;[1 1 1] Client Movement Inputs
  (CallFunction|SMoveUp AxisValue))

(event Input|AxisEvents|InputAxisLookUp
  (params (AxisValue :type Float%20%28single-precision%29))
  ;[1 1 1] Client Movement Inputs
  (CallFunction|SRotPitch AxisValue))

(event Input|AxisEvents|InputAxisTurn
  (params (AxisValue :type Float%20%28single-precision%29))
  ;[1 1 1] Client Movement Inputs
  (CallFunction|SRotYaw AxisValue))

(event Input|AxisEvents|InputAxisRotate
  (params (AxisValue :type Float%20%28single-precision%29))
  ;[1 1 1] Client Movement Inputs
  (CallFunction|SRotRoll AxisValue))

(fn ConstructionScript
  (Variables|/Script/Engine.SpringArmComponent|SetTargetArmLength (Variables|Default|GetSpringArm) (Variables|Camera|GetCameraDistance))
  (Variables|Camera|SetTargetDistance (Variables|Camera|GetCameraDistance))
  (Variables|Camera|SetTargetOffset (Variables|Camera|GetThirdpersonOffset)))

(fn GetClosestInteractable
  (params (Hits :type Array%20of%20Hit%20Result%20Structures))
  (for _array_element Hits
    (if (.bBlockingHit (Collision|BreakHitResult _array_element))
      (if (Utilities|DoesObjectImplementInterface (.HitActor (Collision|BreakHitResult _array_element)) "/Game/SpacePawn/Blueprints/BI_Interact.BI_Interact_C")
        (Utilities|IsValid (LocalVariables|GetTClosest)
          (:Is%20Valid
            (if (< (Math|Vector|VectorLength (- (Transformation|GetActorLocation (.HitActor (Collision|BreakHitResult _array_element))) (.TraceStart (Collision|BreakHitResult _array_element)))) (Math|Vector|VectorLength (- (.TraceStart (Collision|BreakHitResult _array_element)) (Transformation|GetActorLocation (LocalVariables|GetTClosest)))))
              (LocalVariables|SetTClosest (.HitActor (Collision|BreakHitResult _array_element)) :!label _label)
              (LocalVariables|SetTHit _array_element)))
          (:Is%20Not%20Valid
            (goto _label))))))
  (return (LocalVariables|GetTClosest) (LocalVariables|GetTHit)))