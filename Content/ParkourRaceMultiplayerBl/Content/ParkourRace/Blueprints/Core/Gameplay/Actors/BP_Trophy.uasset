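; BP_Trophy is the race's trophy pickup, which decides the winner when a character touches it.
; On the server, the first overlapping BP_Character has its PlayerState stored as WinnerRef in BP_GS_Gameplay.
; A multicast event then plays the poof particle and sound, and the server destroys the trophy.
; A timeline for bobbing the mesh up and down exists, but nothing triggers it.
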(event OnComponentBeginOverlap(SM_Trophy)
  (params (OverlappedComponent :type Primitive%20Component%20Object%20Reference) (OtherActor :type Actor%20Object%20Reference) (OtherComp :type Primitive%20Component%20Object%20Reference) (OtherBodyIndex :type Integer) (bFromSweep :type Boolean) (SweepResult :type Hit%20Result%20Structure%20%28by%20ref%29))
  ;[0.05098 0.05098 0.05098] Set the winner in the Game State upon collision with the Trophy, and call Spawn Poof
  (Networking|SwitchHasAuthority
    (:Authority
      (Utilities|FlowControl|DoOnce false
        (:Completed
          (bind _asbp_character (Utilities|Casting|CastToBP_Character OtherActor))
          (bind _asbp_gs_gameplay (Utilities|Casting|CastToBP_GS_Gameplay (Game|GetGameState)))
          (Variables|/Game/ParkourRace/Blueprints/Core/Gameplay/Core/BP_GS_Gameplay.BP_GS_Gameplay_C|SetWinner_Ref _asbp_gs_gameplay (Variables|/Script/Engine.Pawn|GetPlayerState _asbp_character))
          (CallFunction|MCSpawnPoof))))))

(event Custom|MC_SpawnPoof
  ;[0.05098 0.05098 0.05098] Spawn a poof particle, play poof sound, and destroy actor
  (Niagara|SpawnSystematLocation "/Game/ParkourRace/Assets/Niagara/NS_Poof.NS_Poof" (Transformation|GetActorLocation))
  (Audio|PlaySoundatLocation "/Game/ParkourRace/Assets/Audio/Cues/SC_Poof.SC_Poof" (Transformation|GetActorLocation) "0, 0, 0" 1.5 1.0 0.0 "/Game/ParkourRace/Assets/Audio/Classes/SA_Medium.SA_Medium" "/Game/ParkourRace/Assets/Audio/Classes/SCC_Base.SCC_Base" 0 0)
  (Networking|SwitchHasAuthority
    (:Authority
      (Actor|DestroyActor))))

(fn ConstructionScript)