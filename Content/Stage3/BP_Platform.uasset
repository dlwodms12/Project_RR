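; BP_Platform is a moving platform actor for Stage 3 that travels along the axis of its Arrow component.
; On BeginPlay it caches its start location and plays PlatformTimeLine.
; Each update sets the location to the start plus the Arrow's forward vector, scaled by the timeline's movement value (이동값) and the Direction variable, without sweeping.
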(event EventBeginPlay
  (Variables|Default|SetStartVector (Transformation|GetActorLocation))
  (bind _이동값 (Timeline|PlatformTimeLine Play)
    (:Update
      (Transformation|SetActorLocation (+ (Variables|Default|GetStartVector) (* (Math|Vector|GetForwardVector (Variables|Default|GetArrow)) (* _이동값 (Variables|Default|GetDirection)))) false false))))

(event Collision|EventActorBeginOverlap
  (params (OtherActor :type Actor%20Object%20Reference)))

(event EventTick
  (params (DeltaSeconds :type Float%20%28single-precision%29)))

(fn ConstructionScript)