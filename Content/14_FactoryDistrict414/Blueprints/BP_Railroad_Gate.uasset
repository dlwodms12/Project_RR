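; Railroad crossing gate actor that lowers its arm and animates warning lights when something overlaps a placeholder trigger volume.
; The construction script creates two sets of dynamic materials, main and alternate, on the Gate and Light meshes.
; Three chained timelines run from the overlap: one rolls the gate, and its updates start the others, which drive each set's emissive strength.
; Nothing in the graph raises the gate or stops the lights.
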(event OnComponentBeginOverlap(TriggerVolume)
  (params (OverlappedComponent :type Primitive%20Component%20Object%20Reference) (OtherActor :type Actor%20Object%20Reference) (OtherComp :type Primitive%20Component%20Object%20Reference) (OtherBodyIndex :type Integer) (bFromSweep :type Boolean) (SweepResult :type Hit%20Result%20Structure%20%28by%20ref%29))
  ;[1 1 1] Triggers the animation for train crossing gate to come down. Replace trigger with whatever you need, its a placeholder to showcase its function.
  (bind _newtrack_0 (Timeline|Timeline_0 Play)
    (:Update
      (Transformation|SetRelativeRotation (Variables|Default|GetGate) (Math|Rotator|MakeRotator _newtrack_0 0.0 0.0) false false)
      (bind _newtrack_1 (Timeline|Timeline_1 Play)
        (:Update
          (Rendering|Material|SetScalarParameterValue (Variables|Default|GetGate%20Light) "Emissive Strength" _newtrack_1 :!class /Script/Engine.MaterialInstanceDynamic)
          (bind _newtrack_1_2 (Timeline|Timeline_2 Play)
            (:Update
              (Rendering|Material|SetScalarParameterValue (Variables|Default|GetSings%20Alt) "Emissive Strength" _newtrack_1_2 :!class /Script/Engine.MaterialInstanceDynamic))))))))

(event EventBeginPlay)

(event EventTick
  (params (DeltaSeconds :type Float%20%28single-precision%29)))

(fn ConstructionScript
  (bind _light (Variables|Default|GetLight))
  (bind _gate (Variables|Default|GetGate))
  ;[1 1 1] Toggle for light switch
  (bind _returnvalue (Rendering|Material|CreateDynamicMaterialInstance _light 1 "/Game/14_FactoryDistrict414/Materials/Sign_Extras_mat.Sign_Extras_mat" "None" :!class /Script/Engine.PrimitiveComponent))
  (Variables|Default|SetSigns _returnvalue)
  (bind _returnvalue_2 (Rendering|Material|CreateDynamicMaterialInstance _light 2 "/Game/14_FactoryDistrict414/Materials/Sign_Extras_Alternate.Sign_Extras_Alternate" "None" :!class /Script/Engine.PrimitiveComponent))
  (Variables|Default|SetSings%20Alt _returnvalue_2)
  (bind _returnvalue_3 (Rendering|Material|CreateDynamicMaterialInstance _gate 1 "/Game/14_FactoryDistrict414/Materials/Sign_Extras_mat.Sign_Extras_mat" "None" :!class /Script/Engine.PrimitiveComponent))
  (Variables|Default|SetGate%20Light _returnvalue_3)
  (bind _returnvalue_4 (Rendering|Material|CreateDynamicMaterialInstance _gate 2 0 "None" :!class /Script/Engine.PrimitiveComponent))
  (Variables|Default|SetGate%20Light%20Alt _returnvalue_4))