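; BP_Light_Stand_Base is a configurable work-light stand prop with two housings and two spotlights.
; Its construction script sets the extension's height, optionally randomized, along with its yaw and each housing's roll.
; It gives both housings dynamic material instances, then a toggle drives their emissive strength and the spotlight intensity together.
; All behavior runs at construction; the event graph is empty.
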(event EventBeginPlay)

(event EventActorBeginOverlap
  (params (OtherActor :type Actor%20Object%20Reference)))

(event EventTick
  (params (DeltaSeconds :type Float%20%28single-precision%29)))

(fn ConstructionScript
  (bind _light_stand_extension (Variables|Default|GetLight_Stand_Extension))
  ;[1 1 1] Rotation adjustment for actor
  (if (Variables|Default|GetRandom%20Height)
    (Transformation|SetRelativeLocation _light_stand_extension (Math|Vector|MakeVector 0.0 0.0 (Math|Random|RandomFloatinRange 0.0 1e+02)) false false)
    (else
      (Transformation|SetRelativeLocation _light_stand_extension (Math|Vector|MakeVector 0.0 0.0 (Variables|Default|GetStand%20Height)) false false)))
  (Transformation|SetRelativeRotation _light_stand_extension (Math|Rotator|MakeRotator 0.0 0.0 (Variables|Default|GetStand%20Rotation)) false false)
  ;[1 1 1] Child actor rotation
  (Transformation|SetRelativeRotation (Variables|Default|GetHousing%20A) (Math|Rotator|MakeRotator (Variables|Default|GetHousing%20A%20Rotation) 0.0 0.0) false false)
  (Transformation|SetRelativeRotation (Variables|Default|GetHousing%20B) (Math|Rotator|MakeRotator (Variables|Default|GetHousing%20B%20Rotation) 0.0 0.0) false false)
  ;[1 1 1] Creating dynamic material instances for lights
  (bind _returnvalue (Rendering|Material|CreateDynamicMaterialInstance (Variables|Default|GetHousing%20A) 0 "/Game/14_FactoryDistrict414/Materials/Lights_mat.Lights_mat" "None" :!class /Script/Engine.PrimitiveComponent))
  (Variables|Default|SetDMI%20A _returnvalue)
  (bind _returnvalue_2 (Rendering|Material|CreateDynamicMaterialInstance (Variables|Default|GetHousing%20B) 0 "/Game/14_FactoryDistrict414/Materials/Lights_mat.Lights_mat" "None" :!class /Script/Engine.PrimitiveComponent))
  (Variables|Default|SetDMI%20B _returnvalue_2)
  ;[1 1 1] Toggle for light switch
  (if (Variables|Default|GetLights%20Toggle)
    (Rendering|Material|SetScalarParameterValue (Variables|Default|GetDMI%20A) "Emissive_Strength" 2.0 :!class /Script/Engine.MaterialInstanceDynamic)
    (Rendering|Material|SetScalarParameterValue (Variables|Default|GetDMI%20B) "Emissive_Strength" 2.0 :!class /Script/Engine.MaterialInstanceDynamic)
    (Rendering|Components|Light|SetIntensity (Variables|Default|GetSpotLight1) (Variables|Default|GetLights%20Intesity))
    (else
      (Rendering|Material|SetScalarParameterValue (Variables|Default|GetDMI%20A) "Emissive_Strength" 0.0 :!class /Script/Engine.MaterialInstanceDynamic)
      (Rendering|Material|SetScalarParameterValue (Variables|Default|GetDMI%20B) "Emissive_Strength" 0.0 :!class /Script/Engine.MaterialInstanceDynamic)
      (Rendering|Components|Light|SetIntensity (Variables|Default|GetSpotLight) 0.0))))