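; BP_Light_Floor_Base is a floor light fixture for the Factory District level, with a housing mesh and a spotlight.
; The construction script sets the housing's roll from a Rotation variable and creates a dynamic material instance on its first material slot.
; A LightsToggle flag switches both the material's emissive strength and the spotlight intensity on or off.
; All setup happens at construction, with no active runtime logic.
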(event EventBeginPlay)

(event EventActorBeginOverlap
  (params (OtherActor :type Actor%20Object%20Reference)))

(event EventTick
  (params (DeltaSeconds :type Float%20%28single-precision%29)))

(fn ConstructionScript
  (bind _spotlight (Variables|Default|GetSpotLight))
  ;[1 1 1] Creating dynamic material instances for lights
  (Transformation|SetRelativeRotation (Variables|Default|GetLight_Floor_Housing) (Math|Rotator|MakeRotator (Variables|Default|GetRotation) 0.0 0.0) false false)
  (bind _returnvalue (Rendering|Material|CreateDynamicMaterialInstance (Variables|Default|GetLight_Floor_Housing) 0 "/Game/14_FactoryDistrict414/Materials/Lights_mat.Lights_mat" "None" :!class /Script/Engine.PrimitiveComponent))
  (Variables|Default|SetDMI _returnvalue)
  ;[1 1 1] Toggle for light switch
  (if (Variables|Default|GetLights%20Toggle)
    (Rendering|Material|SetScalarParameterValue (Variables|Default|GetDMI) "Emissive_Strength" 2.0 :!class /Script/Engine.MaterialInstanceDynamic)
    (Rendering|Components|Light|SetIntensity _spotlight (Variables|Default|GetLight%20Intensity))
    (else
      (Rendering|Material|SetScalarParameterValue (Variables|Default|GetDMI) "Emissive_Strength" 0.0 :!class /Script/Engine.MaterialInstanceDynamic)
      (Rendering|Components|Light|SetIntensity _spotlight 0.0))))