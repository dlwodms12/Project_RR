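; BP_Light_Wall_A is a wall light fixture made of a static mesh and a point light, switchable on or off per instance.
; The construction script creates a dynamic material instance on the mesh's first slot from the lights material.
; LightsToggle drives both the material's emissive strength and the point light's intensity, zeroing both when off.
; The event graph is empty, so nothing changes at runtime.
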(event EventBeginPlay)

(event Collision|EventActorBeginOverlap
  (params (OtherActor :type Actor%20Object%20Reference)))

(event EventTick
  (params (DeltaSeconds :type Float%20%28single-precision%29)))

(fn ConstructionScript
  (bind _pointlight (Variables|Default|GetPointLight))
  ;[1 1 1] Creating dynamic material instances for lights
  (bind _returnvalue (Rendering|Material|CreateDynamicMaterialInstance (Variables|Default|GetStaticMesh) 0 "/Game/14_FactoryDistrict414/Materials/Lights_mat.Lights_mat" "None" :!class /Script/Engine.PrimitiveComponent))
  (Variables|Default|SetNewVar_0 _returnvalue)
  ;[1 1 1] Switch for lights
  (if (Variables|Default|GetLights_Toggle)
    (Rendering|Material|SetScalarParameterValue (Variables|Default|GetNewVar_0) "Emissive_Strength" 2.0 :!class /Script/Engine.MaterialInstanceDynamic)
    (Rendering|Components|Light|SetIntensity _pointlight (Variables|Default|GetLight%20Intesity))
    (else
      (Rendering|Material|SetScalarParameterValue (Variables|Default|GetNewVar_0) "Emissive_Strength" 0.0 :!class /Script/Engine.MaterialInstanceDynamic)
      (Rendering|Components|Light|SetIntensity _pointlight 0.0))))