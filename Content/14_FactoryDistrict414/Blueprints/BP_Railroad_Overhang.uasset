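; BP_Railroad_Overhang is a railroad crossing overhang prop with flashing sign lights, driven by a placeholder trigger volume.
; The construction script creates two dynamic instances of Sign_Extras_mat on separate Overhang material slots.
; On overlap, a timeline animates the first instance's Emissive Strength and calls play on a second timeline from its update, which animates the other instance.
; Despite a comment mentioning a gate animation, only emissive values change here.
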(event OnComponentBeginOverlap(TriggerVolume)
  (params (OverlappedComponent :type Primitive%20Component%20Object%20Reference) (OtherActor :type Actor%20Object%20Reference) (OtherComp :type Primitive%20Component%20Object%20Reference) (OtherBodyIndex :type Integer) (bFromSweep :type Boolean) (SweepResult :type Hit%20Result%20Structure%20%28by%20ref%29))
  ;[1 1 1] Triggers the animation for train crossing gate to come down. Replace trigger with whatever you need, its a placeholder to showcase its function.
  (bind _newtrack_1 (Timeline|Timeline_1 Play)
    (:Update
      (Rendering|Material|SetScalarParameterValue (Variables|Default|GetSigns) "Emissive Strength" _newtrack_1 :!class /Script/Engine.MaterialInstanceDynamic)
      (bind _newtrack_1_2 (Timeline|Timeline_2 Play)
        (:Update
          (Rendering|Material|SetScalarParameterValue (Variables|Default|GetSings%20Alt) "Emissive Strength" _newtrack_1_2 :!class /Script/Engine.MaterialInstanceDynamic))))))

(event EventBeginPlay)

(event EventTick
  (params (DeltaSeconds :type Float%20%28single-precision%29)))

(fn ConstructionScript
  (bind _overhang (Variables|Default|GetOverhang))
  ;[1 1 1] Creating dynamic material instances for lights flashing
  (bind _returnvalue (Rendering|Material|CreateDynamicMaterialInstance _overhang 1 "/Game/14_FactoryDistrict414/Materials/Sign_Extras_mat.Sign_Extras_mat" "None" :!class /Script/Engine.PrimitiveComponent))
  (Variables|Default|SetSigns _returnvalue)
  (bind _returnvalue_2 (Rendering|Material|CreateDynamicMaterialInstance _overhang 2 "/Game/14_FactoryDistrict414/Materials/Sign_Extras_mat.Sign_Extras_mat" "None" :!class /Script/Engine.PrimitiveComponent))
  (Variables|Default|SetSings%20Alt _returnvalue_2))