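; BP_Elephant_Turret is a turret that turns toward the player character and fires elephant bullets at it.
; Each PawnSensing sighting of a BP_CustomMoveThirdPersonCharacter snaps the actor's rotation to face that pawn.
; A five-second Delay, which ignores repeat triggers while pending, throttles firing.
; It then spawns BP_Elephant_Bullet at the Arrow's transform, with an explosion emitter there and an elephant sound at the turret.
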(event OnSeePawn(PawnSensing)
  (params (Pawn :type Pawn%20Object%20Reference))
  (Utilities|Casting|CastToBP_CustomMoveThirdPersonCharacter Pawn)
  (Transformation|SetActorRotation (Math|Rotator|FindLookatRotation (Transformation|GetActorLocation) (Transformation|GetActorLocation Pawn)))
  (Utilities|FlowControl|Delay 5.0)
  (Game|SpawnActorfromClass "/Game/Turret/BP_Elephant_Bullet.BP_Elephant_Bullet_C" (Transformation|GetWorldTransform (Variables|Default|GetArrow)) "Undefined" "MultiplyWithRoot" 0 0)
  (Effects|SpawnEmitteratLocation "/Game/StarterContent/Particles/P_Explosion.P_Explosion" (Transformation|GetWorldLocation (Variables|Default|GetArrow)) "0, 0, 0" "0.500000,0.500000,0.500000")
  (Audio|PlaySoundatLocation "/Game/Sound/SoundEffect/Elephant.Elephant" (Transformation|GetActorLocation) "0, 0, 0" 1.0 1.0 0.0 0 0 0 0))

(fn ConstructionScript)