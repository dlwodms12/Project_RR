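; Bear turret for stage 1 that fires cannon projectiles at the player character when it sees one.
; PawnSensing sightings of BP_CustomMoveThirdPersonCharacter snap the whole actor to face that pawn.
; A seven-second Delay, which ignores retriggers while pending, spaces out the shots.
; Each shot spawns a BP_Bear_Bullet and a half-scale explosion effect at the Arrow component, plus a cannon sound at the turret.
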(event OnSeePawn(PawnSensing)
  (params (Pawn :type Pawn%20Object%20Reference))
  (Utilities|Casting|CastToBP_CustomMoveThirdPersonCharacter Pawn)
  (Transformation|SetActorRotation (Math|Rotator|FindLookatRotation (Transformation|GetActorLocation) (Transformation|GetActorLocation Pawn)))
  ;[1 1 1] 대포 쏘는 간극 조절
  (Utilities|FlowControl|Delay 7.0)
  (Game|SpawnActorfromClass "/Game/Turret/BP_Bear_Bullet.BP_Bear_Bullet_C" (Transformation|GetWorldTransform (Variables|Default|GetArrow)) "Undefined" "MultiplyWithRoot" 0 0)
  (Effects|SpawnEmitteratLocation "/Game/StarterContent/Particles/P_Explosion.P_Explosion" (Transformation|GetWorldLocation (Variables|Default|GetArrow)) "0, 0, 0" "0.500000,0.500000,0.500000")
  (Audio|PlaySoundatLocation "/Game/Sound/SoundEffect/SmallCannonSound.SmallCannonSound" (Transformation|GetActorLocation) "0, 0, 0" 1.0 1.0 0.0 0 0 0 0))

(fn ConstructionScript)