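; BP_fan_01 is an animated fan prop with optional spinning blades and an oscillating head.
; On BeginPlay, the Animate flag swaps the static blade for a skeletal mesh whose play rate sets blade speed, or shows the static blade instead.
; With HeadRotate also on, a timeline drives the head's relative yaw at its own speed.
; When animated, the construction script sets head and static blade mobility to Movable or Static based on HeadRotate.
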(event EventBeginPlay
  (bind _skeletalmesh (Variables|Default|GetSkeletalMesh))
  (bind _sm_fan_blade_01 (Variables|Default|GetSM_fan_blade_01))
  (if (Variables|Default|GetAnimate)
    (Utilities|FlowControl|Sequence
      (:then_0
        (Rendering|SetVisibility _sm_fan_blade_01 false false)
        (Rendering|SetVisibility _skeletalmesh true false)
        (Components|Timeline|SetPlayRate _skeletalmesh (Variables|Default|Getblade%20rotate%20speed)))
      (:then_1
        (if (Variables|Default|Gethead_rotate)
          (Components|Timeline|SetPlayRate (Variables|Default|Getrotate) (Variables|Default|Gethead_rotate_speed))
          (bind _angle (Timeline|rotate Play)
            (:Update
              (Transformation|SetRelativeRotation (Variables|Default|GetSM_fan_head_01) (Math|Rotator|MakeRotator 0.0 0.0 _angle) false false))))))
    (else
      (Rendering|SetVisibility _skeletalmesh false false)
      (Rendering|SetVisibility _sm_fan_blade_01 true false))))

(fn ConstructionScript
  (bind _sm_fan_head_01 (Variables|Default|GetSM_fan_head_01))
  (if (Variables|Default|GetAnimate)
    (if (Variables|Default|Gethead_rotate)
      (Transformation|SetMobility _sm_fan_head_01 "Movable")
      (else
        (Transformation|SetMobility _sm_fan_head_01 "Static")))))