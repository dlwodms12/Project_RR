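; BP_fan_05 is a fan prop that shows either an animated or a still blade, chosen by an Animate flag.
; The construction script sets the static blade mesh's mobility to Movable when animated and Static otherwise.
; On BeginPlay it shows either the skeletal mesh, with play rate set from BladeRotateSpeed, or the static blade mesh, and hides the other.
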(event EventBeginPlay
  (bind _skeletalmesh (Variables|Default|GetSkeletalMesh))
  (bind _sm_fan_blade_01 (Variables|Default|GetSM_fan_blade_01))
  (if (Variables|Default|GetAnimate)
    (Rendering|SetVisibility _sm_fan_blade_01 false false)
    (Rendering|SetVisibility _skeletalmesh true false)
    (Components|Timeline|SetPlayRate _skeletalmesh (Variables|Default|Getblade%20rotate%20speed))
    (else
      (Rendering|SetVisibility _skeletalmesh false false)
      (Rendering|SetVisibility _sm_fan_blade_01 true false))))

(fn ConstructionScript
  (bind _sm_fan_blade_01 (Variables|Default|GetSM_fan_blade_01))
  (if (Variables|Default|GetAnimate)
    (Transformation|SetMobility _sm_fan_blade_01 "Movable")
    (else
      (Transformation|SetMobility _sm_fan_blade_01 "Static"))))